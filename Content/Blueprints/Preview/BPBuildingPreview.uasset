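; Placement preview actor for buildings that validates a spot and swaps itself for the real building.
; Overlaps set a blocked flag and deny material, while a downward trace each tick tracks ground contact, both feeding a spawn check.
; Placement separately compares the controller's resources against the DT_Buildings row, then spawns the building and destroys the preview, or shows an error.
; Cursor hover toggles custom depth on the mesh.
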(event `self.ReceiveBeginPlay`
  ;[1 1 1] beginPlay
  (`/Engine/EditorBlueprintResources/StandardMacros.IsValid` (`self.ControllerRef`)
    (:`Is Valid`)
    (:`Is Not Valid`
      (bind _asbpriot_controller (cast `/Game/Blueprints/Player/BPRiotController` (`GameplayStatics.GetPlayerController` 0)))
      (set `self.ControllerRef` _asbpriot_controller))))

(event `self.ReceiveActorEndOverlap`
  (params (OtherActor :type "Actor Object Reference"))
  ;[1 1 1] Overlap
  (if (== (`KismetArrayLibrary.Array_Length` (`self.GetOverlappingActors` null)) 0)
    (`PrimitiveComponent.SetMaterial` (`self.PreviewMesh`) 0 "/Game/Materials/s_preview.s_preview")
    (set `self.Blocked` false)))

(event `self.ReceiveActorBeginOverlap`
  (params (OtherActor :type "Actor Object Reference"))
  ;[1 1 1] Overlap
  (`PrimitiveComponent.SetMaterial` (`self.PreviewMesh`) 0 "/Game/Materials/Deny.Deny")
  (set `self.Blocked` true))

(event `self.ReceiveTick`
  (params (DeltaSeconds :type "Float (single-precision)"))
  (bind _returnvalue (`self.K2_GetActorLocation`))
  ;[1 1 1] Tick
  (bind _outhit (`KismetSystemLibrary.LineTraceSingle` (+ _returnvalue (0.0 0.0 50.0)) (+ _returnvalue (* (`self.GetActorUpVector`) -75.0)) "TraceTypeQuery3"))
  (if (`GameplayStatics.BreakHitResult` _outhit)
    (set `self.OnGround` true)
    (else
      (set `self.OnGround` false))))

(event `self.PreviewMesh.OnBeginCursorOver`
  (params (TouchedComponent :type "PrimitiveComponent Object Reference"))
  ;[1 1 1] MouseOver
  (`PrimitiveComponent.SetRenderCustomDepth` (`self.PreviewMesh`) true))

(event `self.PreviewMesh.OnEndCursorOver`
  (params (TouchedComponent :type "PrimitiveComponent Object Reference"))
  ;[1 1 1] MouseOver
  (`PrimitiveComponent.SetRenderCustomDepth` (`self.PreviewMesh`) false))

(fn `fnPlaceNewBuilding`
  (params (ClassIn :type "/Game/Blueprints/Buildings/BPBuildingMaster Class Reference") (TransformIn :type "Transform Structure"))
  (returns (Success :type Boolean))
  (bind _buildingindex (`self.BuildingIndex`))
  ;[1 1 1] PlaceNewBuilding
  (bind _allowed (`self.fnRequiredResourcesCheck` _buildingindex))
  (if _allowed
    (bind _returnvalue (`|SpawnActorFromClass` ClassIn TransformIn "Undefined" "OverrideRootScale" null _buildingindex))
    (`/Game/Blueprints/Buildings/BPBuildingMaster.OnSpawned` _returnvalue)
    (`self.K2_DestroyActor`)
    (return true)
    (else
      (message `/Game/Interfaces/I_HUDInstructions.ShowErrorInterface` (`BlueprintMapLibrary.Map_Find` (`/Game/Blueprints/Player/BPRiotController.UserWidgets` (`self.ControllerRef`)) "/Game/Blueprints/Widgets/WError.WError_C") "Not enough Resources")
      (return false))))

(fn `fnRequiredResourcesCheck`
  (params (RowIn :type "/Game/ENums/Enum_buildingsRowNames Enum"))
  (returns (Allowed :type Boolean))
  (locals (Allowed_Loc :type Boolean :default true))
  (bind _returnvalue (`|GetDataTableRow` "/Game/DataTables/DT_Buildings.DT_Buildings" (`KismetStringLibrary.Conv_StringToName` (`|GetEnumeratorNameAsString` (enumliteral `/Game/ENums/Enum_buildingsRowNames` RowIn))))
    (:`then`
      (for _array_element (`.BuildingRequiredResources_43_16ECF3C946C5ABD7F8FEC59BAF30D635` (break `/Game/Structs/Building_Properties_Struct` _returnvalue))
        (bind (_resindex _resindexamount) (break `/Game/Structs/STRUCT_ResourcesIndexes` _array_element))
        (if (< (`BlueprintMapLibrary.Map_Find` (`/Game/Blueprints/Player/BPRiotController.ResourceList` (`self.ControllerRef`)) _resindex) _resindexamount)
          (set `local.Allowed_Loc` false)
          (break)))
      (return (`local.Allowed_Loc`)))))

(fn `fnSpawnBuildingCheck`
  (returns (Success :type Boolean))
  (if (and (not (`self.Blocked`)) (`self.OnGround`))
    (return true)
    (else
      (return false))))

(fn `UserConstructionScript`)