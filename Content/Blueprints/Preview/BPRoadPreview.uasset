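; Preview actor for road placement, showing a prospective curved road segment as a single spline mesh.
; Setters move start, mid and end points, deriving tangents from the midpoint, with a flattened, π/2-scaled end tangent and a lockable start tangent.
; SpawnRoad passes the spline's positions and tangents to BPRiotController's AppendRoad when unblocked and given a valid road.
; Overlap-based blocking logic is disconnected, so Blocked never changes here.
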(event `self.ReceiveActorBeginOverlap`
  (params (OtherActor :type "Actor Object Reference")))

(event `self.ReceiveActorEndOverlap`
  (params (OtherActor :type "Actor Object Reference")))

(event `self.ReceiveBeginPlay`
  (`/Engine/EditorBlueprintResources/StandardMacros.IsValid` (`self.ControllerRef`)
    (:`Is Not Valid`
      (set `self.ControllerRef` (cast `/Game/Blueprints/Player/BPRiotController` (`GameplayStatics.GetPlayerController` 0) :!pure true)))))

(fn `info`
  (returns (Pos1 :type "Vector Structure") (Tan1 :type "Vector Structure") (Pos2 :type "Vector Structure") (Tan2 :type "Vector Structure") (Mid :type "Vector Structure"))
  (bind _roadspline (`self.RoadSpline`))
  (return (`SplineMeshComponent.GetStartPosition` _roadspline) (`SplineMeshComponent.GetStartTangent` _roadspline) (`SplineMeshComponent.GetEndPosition` _roadspline) (`SplineMeshComponent.GetEndTangent` _roadspline) (`self.MidPoint`)))

(fn `SetEndPoint`
  (params (End :type "Vector Structure"))
  (`SplineMeshComponent.SetEndPosition` (`self.RoadSpline`) End true)
  (`self.UpdateTangents`))

(fn `SetMidPoint`
  (params (Mid :type "Vector Structure") (SetEnd :type Boolean))
  (bind _output_get (set `self.MidPoint` Mid))
  (if SetEnd
    (`self.SetEndPoint` _output_get))
  (`self.UpdateTangents`))

(fn `SetStartPoint`
  (params (Start :type "Vector Structure"))
  (`SplineMeshComponent.SetStartPosition` (`self.RoadSpline`) Start true)
  (`self.UpdateTangents`))

(fn `SetStartTangent`
  (params (Tangent :type "Vector Structure"))
  (set `self.LockTangent` true)
  (`SplineMeshComponent.SetStartTangent` (`self.RoadSpline`) Tangent true))

(fn `SpawnRoad`
  (params (Add :type "/Game/Blueprints/Buildings/BPRoad Object Reference"))
  (bind _roadspline (`self.RoadSpline`))
  (if (not (`self.Blocked`))
    (`/Engine/EditorBlueprintResources/StandardMacros.IsValid` Add
      (:`Is Valid`
        (`/Game/Blueprints/Player/BPRiotController.AppendRoad` (`self.ControllerRef`) Add (`SplineMeshComponent.GetStartPosition` _roadspline) (`SplineMeshComponent.GetStartTangent` _roadspline) (`SplineMeshComponent.GetEndPosition` _roadspline) (`SplineMeshComponent.GetEndTangent` _roadspline))))))

(fn `UpdateTangents`
  (bind _roadspline (`self.RoadSpline`))
  (bind _midpoint (`self.MidPoint`))
  (bind _roadspline_2 (`self.RoadSpline`))
  (`SplineMeshComponent.SetEndTangent` _roadspline_2 (* (* (- (`SplineMeshComponent.GetEndPosition` _roadspline) _midpoint) (1.0 1.0 0.0)) (/ (`KismetMathLibrary.GetPI`) 2.0)) true)
  (if (not (`self.LockTangent`))
    (`SplineMeshComponent.SetStartTangent` _roadspline_2 (- _midpoint (`SplineMeshComponent.GetStartPosition` _roadspline)) true)))

(fn `UserConstructionScript`)