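; Behavior tree task that reports the controlled human character for a shift at the building stored in its CurrentLocation blackboard key.
; With a valid building, it calls ReportToShift, sets IsBusy, clears TargetLocation and finishes successfully.
; Otherwise it clears TargetLocation and IsBusy and fails.
; An unconnected branch that disables collision and moves to the building remains, marked with a note to switch back.
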(event `self.ReceiveExecuteAI`
  (params (OwnerController :type "AIController Object Reference") (ControlledPawn :type "Pawn Object Reference"))
  (bind _returnvalue (`BTFunctionLibrary.GetBlackboardValueAsObject` (`self.CurrentLocation`)))
  (`/Engine/EditorBlueprintResources/StandardMacros.IsValid` _returnvalue
    (:`Is Valid`
      (`/Game/Blueprints/Buildings/BPBuildingMaster.ReportToShift` (cast `/Game/Blueprints/Buildings/BPBuildingMaster` _returnvalue :!pure true) (cast `/Game/Blueprints/Units/BPMasterHumanChar` ControlledPawn :!pure true))
      (`BTFunctionLibrary.SetBlackboardValueAsBool` (`self.IsBusy`) true)
      (`BTFunctionLibrary.ClearBlackboardValue` (`self.TargetLocation`))
      (`self.FinishExecute` true))
    (:`Is Not Valid`
      (`BTFunctionLibrary.ClearBlackboardValue` (`self.TargetLocation`))
      (`BTFunctionLibrary.SetBlackboardValueAsBool` (`self.IsBusy`))
      (`self.FinishExecute` false))))