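; Behavior tree task that sends an AI unit to work on a building under construction.
; It takes the first entry in the player controller's BuildingsInProgress list, caching that BPRiotController on first use.
; It writes the building's rally point decal location to TargetLocation and the building itself to Destination on the blackboard.
; It succeeds when a building is in progress and fails when the list is empty.
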(event `self.ReceiveExecuteAI`
  (params (OwnerController :type "AIController Object Reference") (ControlledPawn :type "Pawn Object Reference"))
  (bind _playercontrollerref (`self.PlayerControllerRef`))
  (bind _buildingsinprogress (`/Game/Blueprints/Player/BPRiotController.BuildingsInProgress` _playercontrollerref))
  (bind _output (`|GetArrayItem` _buildingsinprogress))
  (`/Engine/EditorBlueprintResources/StandardMacros.IsValid` OwnerController
    (:`Is Valid`
      _)
    (:`Is Not Valid`
      (set `self.Controller` (`self.Controller`))))
  (`/Engine/EditorBlueprintResources/StandardMacros.IsValid` ControlledPawn
    (:`Is Valid`
      _)
    (:`Is Not Valid`
      (set `self.Pawn` (`self.Pawn`))))
  (`/Engine/EditorBlueprintResources/StandardMacros.IsValid` _playercontrollerref
    (:`Is Valid`
      _)
    (:`Is Not Valid`
      (set `self.PlayerControllerRef` (cast `/Game/Blueprints/Player/BPRiotController` (`GameplayStatics.GetPlayerController` 0) :!pure true))))
  (if (> (`KismetArrayLibrary.Array_Length` _buildingsinprogress) 0)
    (`BTFunctionLibrary.SetBlackboardValueAsVector` (`self.TargetLocation`) (`SceneComponent.K2_GetComponentLocation` (`/Game/Blueprints/Buildings/BPBuildingMaster.RallyPointDecal` _output)))
    (`BTFunctionLibrary.SetBlackboardValueAsObject` (`self.Destination`) _output)
    (`self.FinishExecute` true)
    (else
      (`self.FinishExecute` false))))