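; EQS context for human units that supplies their resource deposit as the query's single actor.
; It returns the querier character's CurrentDeposit if it is valid.
; Otherwise it copies CurrentJobDeposit from the industry at the character's place of employment, taken from its profile, into CurrentDeposit and returns that.
; A debug print for a found deposit is left disconnected.
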(fn `ProvideSingleActor`
  (params (QuerierObject :type "Object Object Reference") (QuerierActor :type "Actor Object Reference"))
  (returns (ResultingActor :type "Actor Object Reference"))
  (locals (ResourceToGather_Loc :type "/Game/Blueprints/Resources/BPMasterResource Object Reference"))
  (bind _asbpmaster_human_char (cast `/Game/Blueprints/Units/BPMasterHumanChar` QuerierActor :!pure true))
  (bind _currentdeposit (`/Game/Blueprints/Units/BPMasterHumanChar.CurrentDeposit` _asbpmaster_human_char))
  (`/Engine/EditorBlueprintResources/StandardMacros.IsValid` _currentdeposit
    (:`Is Valid`
      (return _currentdeposit))
    (:`Is Not Valid`
      (bind _output_get (set `/Game/Blueprints/Units/BPMasterHumanChar.CurrentDeposit` (`/Game/Blueprints/Buildings/Industrial/BPIndMaster.CurrentJobDeposit` (cast `/Game/Blueprints/Buildings/Industrial/BPIndMaster` (`.PlaceOfEmployment_17_24FB15DC431FF5690B2068901A922B03` (break `/Game/Structs/UnitProperties` (`/Game/Blueprints/Units/BPMasterHumanChar.MyProfile` _asbpmaster_human_char))) :!pure true)) _asbpmaster_human_char))
      (return _output_get))))