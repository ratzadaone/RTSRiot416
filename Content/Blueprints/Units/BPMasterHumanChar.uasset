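; Master human NPC unit that can gather resources, take jobs and find housing.
; Construction randomizes gender, name and body colour into a profile, which employment and housing functions update through game-state buildings.
; Deposit search writes the nearest resource to the AI blackboard, while gathering itself only prints.
; Hover toggles custom depth, selection lerps the player pawn over before a gated Tick follow, and a scene component yaws toward the camera.
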(event `MyDelay`
  (`KismetSystemLibrary.Delay` 1.0))

(event `self.ReceiveBeginPlay`
  ;[1 1 1] BeginPlay
  (set `self.AIControllerRef` (cast `/Game/Blueprints/Units/BPAIControllerHumanChar` (`AIBlueprintHelperLibrary.GetAIController` self) :!pure true))
  (`/Engine/EditorBlueprintResources/StandardMacros.IsValid` (`self.ControllerRef`)
    (:`Is Valid`)
    (:`Is Not Valid`
      (set `self.ControllerRef` (cast `/Game/Blueprints/Player/BPRiotController` (`GameplayStatics.GetPlayerController` 0) :!pure true)))))

(event `self.ReceiveTick`
  (params (DeltaSeconds :type "Float (single-precision)"))
  (bind (_returnvalue_x _returnvalue_y) (`KismetMathLibrary.BreakVector` (`self.K2_GetActorLocation`)))
  (bind _playerpawnref (`/Game/Blueprints/Player/BPRiotController.PlayerPawnRef` (`self.ControllerRef`)))
  (bind (_returnvalue_x_2 _returnvalue_y_2 _returnvalue_z) (`KismetMathLibrary.BreakVector` (`self.K2_GetActorLocation` _playerpawnref)))
  (bind (_returnvalue_roll _returnvalue_pitch _returnvalue_yaw) (`KismetMathLibrary.BreakRotator` (`KismetMathLibrary.FindLookAtRotation` (`SceneComponent.K2_GetComponentLocation` (`self.Scene`)) (`SceneComponent.K2_GetComponentLocation` (`/Game/Blueprints/Player/BPRiotPawn.Camera` (`/Game/Blueprints/Player/BPRiotController.PlayerPawnRef` (`self.ControllerRef`)))))))
  ;[1 1 1] Tick - set bars rotation
  (`SceneComponent.K2_SetWorldRotation` (`self.Scene`) (`KismetMathLibrary.MakeRotator` 0.0 0.0 _returnvalue_yaw) false false)
  ;[1 1 1] FollowCamera
  (`/Engine/EditorBlueprintResources/StandardMacros.Gate` true :!label _label
    (:`Exit`
      (`self.K2_SetActorLocation` _playerpawnref (`KismetMathLibrary.MakeVector` _returnvalue_x _returnvalue_y _returnvalue_z) false false))))

(event `OpenFollowgate`
  ;[1 1 1] FollowCamera
  (goto _label :!via `Open`))

(event `CloseFollowGate`
  ;[1 1 1] FollowCamera
  (goto _label :!via `Close`))

(event `OnSelect`
  (bind (_direction _newtrack_0) (`Timeline|Timeline_0` :!via `PlayFromStart`)
    (:`Update`
      (`self.K2_SetActorLocation` (`/Game/Blueprints/Player/BPRiotController.PlayerPawnRef` (`self.ControllerRef`)) (`/Game/Blueprints/Functions/BPFunctionLibrary.HUD_LerpLocation` (`self.K2_GetActorLocation` (`/Game/Blueprints/Units/BPAIControllerHumanChar.PawnRef` (`self.AIControllerRef`))) (`self.K2_GetActorLocation`) _newtrack_0) false false))
    (:`Finished`
      (`self.OpenFollowgate`))))

(event `self.CapsuleComponent.OnBeginCursorOver`
  (params (TouchedComponent :type "PrimitiveComponent Object Reference"))
  (`PrimitiveComponent.SetRenderCustomDepth` (`self.Mesh`) true))

(event `self.CapsuleComponent.OnEndCursorOver`
  (params (TouchedComponent :type "PrimitiveComponent Object Reference"))
  (`PrimitiveComponent.SetRenderCustomDepth` (`self.Mesh`) false))

(fn `CheckForEmployment`
  (returns (FoundEmployment :type Boolean))
  (locals (HiringBuildingLocal :type "/Game/Blueprints/Buildings/BPBuildingMaster Object Reference"))
  (bind (_name _type _occupation _placeofemployment _residency) (break `/Game/Structs/UnitProperties` (`self.MyProfile`)))
  (bind (_buildingreference _buildingtype _buildingname _occupationtype) (break `/Game/Structs/Struct_Building` (`/Game/Blueprints/Buildings/BPBuildingMaster.BuildingStruct` (`local.HiringBuildingLocal`))))
  (if (`|EnumEquality` (`.Occupation_15_EE482E7F40133191F94DE5AB7E17D6CB` (break `/Game/Structs/UnitProperties` (`self.MyProfile`))) "NewEnumerator0")
    (bind (_isjobavailable _jobsavailable) (`/Game/Blueprints/Game/BPRiotGameState.GetAvailableJobs` (`/Game/Blueprints/Player/BPRiotController.GameStateRef` (`self.ControllerRef`))))
    (if _isjobavailable
      (bind (_washired _hiringbuilding) (`/Game/Blueprints/Buildings/BPBuildingMaster.HireEmployee` (`|GetArrayItem` _jobsavailable (`KismetMathLibrary.RandomIntegerInRange` 0 (- (`KismetArrayLibrary.Array_Length` _jobsavailable) 1))) self))
      (if _washired
        (set `local.HiringBuildingLocal` _hiringbuilding)
        (set `self.MyProfile` (make `/Game/Structs/UnitProperties` _name _type _occupationtype _buildingreference _residency))
        (return true)
        (else
          (return false)))
      (else
        (return false)))
    (else
      (return false))))

(fn `CheckForHousing`
  (returns (FoundHouse :type Boolean) (House :type "/Game/Blueprints/Buildings/Residential/BPResMaster Object Reference"))
  (locals (FoundHousing_Loc :type Boolean :default false) (Residence_Loc :type "/Game/Blueprints/Buildings/Residential/BPResMaster Object Reference"))
  (bind _buildingsingame (`/Game/Blueprints/Game/BPRiotGameState.BuildingsInGame` (`/Game/Blueprints/Player/BPRiotController.GameStateRef` (`self.ControllerRef`))))
  (bind _values (`BlueprintMapLibrary.Map_Values` _buildingsingame))
  (for (_array_element _array_index) _values
    (switch `/Game/ENums/Enum_BuildingType` _array_element
      (:`NewEnumerator0`
        (bind _keys (`BlueprintMapLibrary.Map_Keys` _buildingsingame))
        (bind _asbpres_master (cast `/Game/Blueprints/Buildings/Residential/BPResMaster` (`|GetArrayItem` _keys _array_index) :!pure true))
        (bind _accepted (`/Game/Blueprints/Buildings/Residential/BPResMaster.ApplyForResidency` _asbpres_master))
        (bind _output_get (set `local.FoundHousing_Loc` _accepted))
        (if _output_get
          (set `local.Residence_Loc` _asbpres_master)
          (break)
          (else
            (set `local.Residence_Loc` null))))))
  (return (`local.FoundHousing_Loc`) (`local.Residence_Loc`)))

(fn `FindDeposit`
  (params (ResourceTypeIn :type Name))
  (locals (LocalValidDeposits :type "Array of /Game/Blueprints/Resources/BPMasterDeposit Object Reference") (Deposit_Loc :type "/Game/Blueprints/Resources/BPMasterDeposit Object Reference") (DistanceToDeposit_Loc :type "Float (double-precision)" :default 0.0))
  (bind _outactors (`GameplayStatics.GetAllActorsOfClass` "/Game/Blueprints/Resources/BPMasterDeposit.BPMasterDeposit_C"))
  (for _array_element _outactors
    (if (and (> (`/Game/Blueprints/Resources/BPMasterDeposit.DepositCurrentCapacity` _array_element) 0) (== "None" ResourceTypeIn))
      (`KismetArrayLibrary.Array_Add` (`local.LocalValidDeposits`) _array_element)))
  (if (> (`KismetArrayLibrary.Array_Length` (`local.LocalValidDeposits`)) 0)
    (for (_array_element_2 _array_index) (`local.LocalValidDeposits`)
      (set `local.Deposit_Loc` _array_element_2)
      (if (== _array_index 0)
        (set `self.CurrentDeposit` (`local.Deposit_Loc`) :!label _label)
        (set `local.DistanceToDeposit_Loc` (`self.GetDistanceTo` (`local.Deposit_Loc`) self))
        (elif (< (`self.GetDistanceTo` (`local.Deposit_Loc`) self) (`local.DistanceToDeposit_Loc`))
          (goto _label))))
    (`self.FindNearResourcesInDeposit`)))

(fn `FindNearResourcesInDeposit`
  (locals (ResourceInDeposit_Loc :type "Array of /Game/Blueprints/Resources/BPMasterResource Object Reference") (Resource_Loc :type "/Game/Blueprints/Resources/BPMasterResource Object Reference") (DistanceToResourceLoc :type "Float (double-precision)" :default 0.0))
  (bind _returnvalue (`AIBlueprintHelperLibrary.GetBlackboard` null))
  (if (> (`/Game/Blueprints/Resources/BPMasterDeposit.DepositCurrentCapacity` (`self.CurrentDeposit`)) 0)
    (bind _output_get (set `local.ResourceInDeposit_Loc` (`/Game/Blueprints/Resources/BPMasterDeposit.ResourceInDeposit` (`self.CurrentDeposit`))))
    (for (_array_element _array_index) _output_get
      (set `local.Resource_Loc` _array_element)
      (if (== _array_index 0)
        (set `self.CurrentResource` (`local.Resource_Loc`) :!label _label)
        (set `local.DistanceToResourceLoc` (`self.GetDistanceTo` (`local.Resource_Loc`) self))
        (elif (< (`self.GetDistanceTo` (`local.Resource_Loc`) self) (`local.DistanceToResourceLoc`))
          (goto _label))))
    (`/Engine/EditorBlueprintResources/StandardMacros.IsValid` _returnvalue
      (:`Is Valid`
        (`BlackboardComponent.SetValueAsObject` _returnvalue (`self.ObjectToPickVarName`) (`self.CurrentResource`))
        (`BlackboardComponent.SetValueAsBool` _returnvalue (`self.IsMovingVarName`) false)))
    (else
      (return))))

(fn `GatherResource`
  (locals (AmountToExtract_Loc :type Integer))
  (`/Engine/EditorBlueprintResources/StandardMacros.IsValid` (`self.CurrentResource`)
    (:`Is Valid`
      (if (<= (+ (`self.CurrentResourceCarry`) (`local.AmountToExtract_Loc`)) (`self.MaxResourceCanCarry`))
        (`KismetSystemLibrary.PrintString` "RESourcegathering")))
    (:`Is Not Valid`
      (`self.FindNearResourcesInDeposit`))))

(fn `GetRandomName`
  (params (Type :type "/Game/ENums/Enum_NPCType Enum"))
  (returns (Name :type String))
  (if (`|EnumEquality` Type "NewEnumerator0")
    (return (`|GetEnumeratorNameAsString` (enumliteral `/Game/ENums/Enum_NPCNameMale` (cast `/Game/ENums/Enum_NPCNameMale` (`KismetMathLibrary.Conv_IntToByte` (`KismetMathLibrary.RandomIntegerInRange` 0 (- (enumcount `/Game/ENums/Enum_NPCNameMale`) 1)))))))
    (else
      (return (`|GetEnumeratorNameAsString` (enumliteral `/Game/ENums/Enum_NPCNameFemale` (cast `/Game/ENums/Enum_NPCNameFemale` (`KismetMathLibrary.Conv_IntToByte` (`KismetMathLibrary.RandomIntegerInRange` 0 (- (enumcount `/Game/ENums/Enum_NPCNameFemale`) 1))))))))))

(fn `LeaveLocation`
  (params (LocationIn :type "Object Object Reference"))
  (returns (ExitSuccess :type Boolean))
  ;[1 0.065 0.065] To Add rest of stuffff - maybe check for each one ???
  (bind _asbpbuilding_master (cast `/Game/Blueprints/Buildings/BPBuildingMaster` LocationIn)
    (:`then`
      (bind _success (`/Game/Blueprints/Buildings/BPBuildingMaster.ExitBuilding` _asbpbuilding_master self))
      (return _success))
    (:`CastFailed`
      (return false))))

(fn `RandomFeatures`
  (locals (MaterialInstance :type "MaterialInstanceDynamic Object Reference") (FemaleColour :type "LinearColor Structure" :default (struct :`R` 0.7 :`G` 0.240857 :`B` 0.490941)) (MaleColour :type "LinearColor Structure" :default (struct :`R` 0.235679 :`G` 0.18766 :`B` 0.7)))
  (bind _materialinstance (`local.MaterialInstance`))
  (bind _returnvalue (`PrimitiveComponent.CreateDynamicMaterialInstance` (`self.Mesh`) 0 "/Game/Materials/M_UE4Man_Body_Inst.M_UE4Man_Body_Inst"))
  (set `local.MaterialInstance` _returnvalue)
  (if (`|EnumEquality` (enumliteral `/Game/ENums/Enum_NPCType` (cast `/Game/ENums/Enum_NPCType` (`KismetMathLibrary.Conv_IntToByte` (`KismetMathLibrary.RandomIntegerInRange` 0 (- (enumcount `/Game/ENums/Enum_NPCType`) 1))))) "NewEnumerator0")
    (`MaterialInstanceDynamic.SetVectorParameterValue` _materialinstance "BodyColor" (`local.MaleColour`))
    (bind _name (`self.GetRandomName` "NewEnumerator0"))
    (set `self.MyProfile` (make `/Game/Structs/UnitProperties` _name))
    (else
      (`MaterialInstanceDynamic.SetVectorParameterValue` _materialinstance "BodyColor" (`local.FemaleColour`))
      (bind _name_2 (`self.GetRandomName` "NewEnumerator1"))
      (set `self.MyProfile` (make `/Game/Structs/UnitProperties` _name_2 "NewEnumerator1")))))

(fn `SetDebugInfo`
  (params (StringIn :type String))
  (locals (LastAction_Loc :type String) (ShowActions_Loc :type String) (Count :type Integer))
  (bind _lastaction_loc (`local.LastAction_Loc`))
  (bind _debugarr (`self.DebugArr`))
  (bind _count (`local.Count`))
  (bind _output_get (set `local.LastAction_Loc` StringIn))
  (if (and (`KismetStringLibrary.NotEqual_StrStr` _output_get) (`KismetStringLibrary.NotEqual_StrStr` (`self.LastAction`) (`local.LastAction_Loc`)))
    (`KismetArrayLibrary.Array_Add` _debugarr _lastaction_loc)
    (set `self.LastAction` _lastaction_loc)
    (bind (_arrayindex _arrayelement) (`/Engine/EditorBlueprintResources/StandardMacros.ReverseForEachLoop` _debugarr)
      (:`LoopBody`
        (`/Engine/EditorBlueprintResources/StandardMacros.IncrementInt` _count
          (:`  `
            (if (< _count 21)
              (set `local.ShowActions_Loc` (`KismetStringLibrary.Concat_StrStr` (`local.ShowActions_Loc`) " \n" _arrayelement))))))
      (:`Completed`
        (`TextBlock.SetText` (`/Game/Blueprints/Widgets/WUnitHumanSingle.MultipleActions` (cast `/Game/Blueprints/Widgets/WUnitHumanSingle` (`BlueprintMapLibrary.Map_Find` (`/Game/Blueprints/Player/BPRiotController.UserWidgets` (`self.ControllerRef`)) "/Game/Blueprints/Widgets/WUnitHumanSingle.WUnitHumanSingle_C") :!pure true)) (`KismetTextLibrary.Conv_StringToText` (`local.ShowActions_Loc`)))))))

(fn `SetIsBusy`
  (params (IsBusy :type Boolean))
  (`BlackboardComponent.SetValueAsBool` (`AIBlueprintHelperLibrary.GetBlackboard` (`self.AIControllerRef`)) (`self.IsBusyVarName`) IsBusy)
  (return))

(fn `SetNewHouse`
  (params (HouseIn :type "Actor Object Reference"))
  (bind (_name _type _occupation _placeofemployment) (break `/Game/Structs/UnitProperties` (`self.MyProfile`)))
  (bind _asbpres_master (cast `/Game/Blueprints/Buildings/Residential/BPResMaster` HouseIn)
    (:`then`
      (set `self.MyProfile` (make `/Game/Structs/UnitProperties` _name _type _occupation _placeofemployment _asbpres_master))
      (return))
    (:`CastFailed`
      (`KismetSystemLibrary.PrintString` "NEW RESIDENCY FAILED" true true (struct :`R` 1.0 :`B` 0.109699 :`A` 1.0) 20.0))))

(fn `UserConstructionScript`
  (`self.RandomFeatures`))