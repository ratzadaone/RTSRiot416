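; AI controller for human units, running their behavior tree and holding needs, coins and worked-time state.
; Looping timers scaled by game speed deplete or regenerate stamina and update the pawn's bar; another increments WorkedHours every second.
; PayRent and GetPayed move money between the unit and the player's resource list, using the blackboard's house for rent and refreshing a hardcoded main UI slot.
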(event `SwitchSleep`
  (bind _returnvalue (/ (`/Game/Blueprints/Game/BPRiotGameState.DefaultGameSpeed` (`self.GameStateRef`)) 60.0))
  ;[1 1 1] BeginPlay
  (if (`KismetSystemLibrary.K2_IsTimerPausedHandle` (`self.StaminaDepleteHandle`)) :!label _label
    (bind _returnvalue_2 (`KismetSystemLibrary.K2_SetTimer` null "RegainStamina" _returnvalue true))
    (set `self.StaminaRegenHandle` _returnvalue_2)
    (else
      (bind _returnvalue_3 (`KismetSystemLibrary.K2_SetTimer` null "DepleteStamina" _returnvalue true))
      (set `self.StaminaDepleteHandle` _returnvalue_3))))

(event `self.ReceiveBeginPlay`
  ;[1 1 1] BeginPlay
  (`/Engine/EditorBlueprintResources/StandardMacros.IsValid` null
    (:`Is Valid`
      _)
    (:`Is Not Valid`
      (set `self.PlayerControllerRef` (cast `/Game/Blueprints/Player/BPRiotController` (`GameplayStatics.GetPlayerController` 0) :!pure true))))
  (`/Engine/EditorBlueprintResources/StandardMacros.IsValid` (`self.GameStateRef`)
    (:`Is Valid`
      _)
    (:`Is Not Valid`
      (set `self.GameStateRef` (cast `/Game/Blueprints/Game/BPRiotGameState` (`GameplayStatics.GetGameState`) :!pure true))))
  (`self.RunBehaviorTree` "/Game/Blueprints/Units/BTHumanChar.BTHumanChar")
  (goto _label))

(event `self.OnPossess`
  (params (PossessedPawn :type "Pawn Object Reference"))
  ;[1 1 1] OnPossess
  (set `self.PawnRef` (cast `/Game/Blueprints/Units/BPMasterHumanChar` PossessedPawn :!pure true))
  (bind _returnvalue (`KismetSystemLibrary.K2_SetTimerDelegate` (delegate `CheckIfWorking`) 1.0 true))
  (set `self.WorkHandle` _returnvalue))

(event `CheckIfWorking`
  ;[1 1 1] OnPossess
  (bind _result (`/Engine/EditorBlueprintResources/StandardMacros.IncrementFloat` (`self.WorkedHours`))
    (:`  `
      (`KismetSystemLibrary.PrintString` (`KismetStringLibrary.Conv_DoubleToString` _result)))))

(event `self.ReceiveTick`
  (params (DeltaSeconds :type "Float (single-precision)")))

(fn `DepleteStamina`
  (set `self.Stamina` (`KismetMathLibrary.FClamp` (- (`self.Stamina`) (/ (`self.StaminaDepleteHour`) 60.0)) 0.0 100.0))
  (`ProgressBar.SetPercent` (`/Game/Blueprints/Widgets/WUnitBars.StaminaBar` (cast `/Game/Blueprints/Widgets/WUnitBars` (`WidgetComponent.GetUserWidgetObject` (`/Game/Blueprints/Units/BPMasterHumanChar.WidgetBars` (`self.PawnRef`))) :!pure true)) (/ (`self.Stamina`) 100.0)))

(fn `GetNeeds`
  (returns (Stamina :type "Float (double-precision)") (Hunger :type "Float (double-precision)") (Happiness :type "Float (double-precision)") (RiotLevel :type "Float (double-precision)"))
  (return (`self.Stamina`) (`self.Hunger`) (`self.Happiness`) (`self.RiotLevel`)))

(fn `GetPayed`
  (returns (Payed :type Boolean))
  (bind _resourcelist (`/Game/Blueprints/Player/BPRiotController.ResourceList` (`self.PlayerControllerRef`)))
  (bind _returnvalue (/ (`self.WorkedHours`) (`/Game/Blueprints/Game/BPRiotGameState.DefaultGameSpeed` (`self.GameStateRef`))))
  (bind _returnvalue_2 (`KismetMathLibrary.Conv_IntToDouble` (`BlueprintMapLibrary.Map_Find` _resourcelist "NewEnumerator2")))
  (`/Game/Blueprints/Units/BPMasterHumanChar.SetDebugInfo` (`self.PawnRef`) (`KismetStringLibrary.Concat_StrStr` "WillGet Payedfor: " (`KismetStringLibrary.Conv_DoubleToString` (`self.WorkedHours`))))
  (`BlueprintMapLibrary.Map_Add` _resourcelist "NewEnumerator2" (`KismetMathLibrary.FCeil` (+ (* _returnvalue -1.0) _returnvalue_2)))
  (`TextBlock.SetText` (`/Game/Blueprints/Widgets/WidgetElements/ResourceInfo.ResourceText` (`|GetArrayItem` (`/Game/Blueprints/Widgets/WMainUI.ResourceInfoWidgets` (cast `/Game/Blueprints/Widgets/WMainUI` (`BlueprintMapLibrary.Map_Find` (`/Game/Blueprints/Player/BPRiotController.UserWidgets` (`self.PlayerControllerRef`)) "/Game/Blueprints/Widgets/WMainUI.WMainUI_C") :!pure true)) 4)) (`KismetTextLibrary.Conv_DoubleToText` _returnvalue_2 "HalfToEven"))
  (set `self.Coins` (+ (`KismetMathLibrary.Conv_IntToDouble` (`KismetMathLibrary.FCeil` _returnvalue)) (`self.Coins`)))
  (set `self.WorkedHours` 0.0)
  (return true))

(fn `PayRent`
  (params (IsRefund :type Boolean))
  (returns (Payed :type Boolean))
  (locals (CostLoc :type "Float (double-precision)"))
  (bind _costloc (`local.CostLoc`))
  (bind _coins (`self.Coins`))
  (bind _returnvalue (`BlackboardComponent.GetValueAsObject` (`self.Blackboard`) "HouseReference"))
  (bind _resourcelist (`/Game/Blueprints/Player/BPRiotController.ResourceList` (`self.PlayerControllerRef`)))
  (bind _returnvalue_2 (`KismetMathLibrary.Conv_IntToDouble` (`BlueprintMapLibrary.Map_Find` _resourcelist "NewEnumerator2")))
  (bind _rentcost (`/Game/Blueprints/Buildings/Residential/BPResMaster.RentCost` (cast `/Game/Blueprints/Buildings/Residential/BPResMaster` _returnvalue :!pure true)))
  (`/Engine/EditorBlueprintResources/StandardMacros.IsValid` _returnvalue
    (:`Is Valid`
      (if IsRefund
        (set `local.CostLoc` (* _rentcost -1.0))
        (else
          (set `local.CostLoc` _rentcost)))
      (if (> _coins _costloc)
        (`/Game/Blueprints/Units/BPMasterHumanChar.SetDebugInfo` (`self.PawnRef`) (`KismetStringLibrary.Concat_StrStr` "Payed rent: " (`KismetStringLibrary.Conv_DoubleToString` _costloc)))
        (set `self.Coins` (+ _coins (* (`local.CostLoc`) -1.0)))
        (`BlueprintMapLibrary.Map_Add` _resourcelist "NewEnumerator2" (`KismetMathLibrary.FTrunc` (+ (`local.CostLoc`) _returnvalue_2)))
        (`TextBlock.SetText` (`/Game/Blueprints/Widgets/WidgetElements/ResourceInfo.ResourceText` (`|GetArrayItem` (`/Game/Blueprints/Widgets/WMainUI.ResourceInfoWidgets` (cast `/Game/Blueprints/Widgets/WMainUI` (`BlueprintMapLibrary.Map_Find` (`/Game/Blueprints/Player/BPRiotController.UserWidgets` (`self.PlayerControllerRef`)) "/Game/Blueprints/Widgets/WMainUI.WMainUI_C") :!pure true)) 4)) (`KismetTextLibrary.Conv_DoubleToText` _returnvalue_2 "HalfToEven"))
        (return true)
        (else
          (return false))))
    (:`Is Not Valid`
      (return false))))

(fn `RegainStamina`
  (set `self.Stamina` (`KismetMathLibrary.FClamp` (+ (`self.Stamina`) (/ (`self.StaminaRegenHour`) 60.0)) 0.0 100.0))
  (`ProgressBar.SetPercent` (`/Game/Blueprints/Widgets/WUnitBars.StaminaBar` (cast `/Game/Blueprints/Widgets/WUnitBars` (`WidgetComponent.GetUserWidgetObject` (`/Game/Blueprints/Units/BPMasterHumanChar.WidgetBars` (`self.PawnRef`))) :!pure true)) (/ (`self.Stamina`) 100.0))
  (return))

(fn `UserConstructionScript`)