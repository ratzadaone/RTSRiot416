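; Behavior tree decorator that checks the storage of the mine where an AI human character works.
; The AI check caches the controlled BPMasterHumanChar, then casts its profile's PlaceOfEmployment to BP_Ind_Mine.
; Despite the MineFull name, it passes while the mine's internal storage is below maximum.
; The non-AI condition check always returns false.
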(fn `PerformConditionCheck`
  (params (OwnerActor :type "Actor Object Reference"))
  (returns (ReturnValue :type Boolean))
  (return false))

(fn `PerformConditionCheckAI`
  (params (OwnerController :type "AIController Object Reference") (ControlledPawn :type "Pawn Object Reference"))
  (returns (ReturnValue :type Boolean))
  ;[1 1 1] pawnCast
  (`/Engine/EditorBlueprintResources/StandardMacros.IsValid` (`self.Pawn`)
    (:`Is Valid`
      _)
    (:`Is Not Valid`
      (bind _output_get (set `self.Pawn` (cast `/Game/Blueprints/Units/BPMasterHumanChar` ControlledPawn :!pure true)))))
  (bind (_myprofile_name _myprofile_type _myprofile_occupation _myprofile_placeofemployment) (break `/Game/Structs/UnitProperties` (`/Game/Blueprints/Units/BPMasterHumanChar.MyProfile` _output_get)))
  (bind _asbp_ind_mine (cast `/Game/Blueprints/Buildings/Industrial/BP_Ind_Mine` _myprofile_placeofemployment :!pure true))
  (return (< (`/Game/Blueprints/Buildings/Industrial/BPIndMaster.CurrentInternalStorage` _asbp_ind_mine) (`/Game/Blueprints/Buildings/Industrial/BPIndMaster.MaxInternalStorage` _asbp_ind_mine))))