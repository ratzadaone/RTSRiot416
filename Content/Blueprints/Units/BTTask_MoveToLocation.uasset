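; Behavior tree task that moves a unit to the blackboard TargetLocation vector using AI MoveTo with a wide acceptance radius.
; On success it copies the Destination object into CurrentLocation, clears Destination and finishes successfully.
; A blocked move retries, while an aborted or invalid one fails the task.
; Aborting stops movement, clears all three location keys and finishes the abort.
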(event `self.ReceiveExecuteAI`
  (params (OwnerController :type "AIController Object Reference") (ControlledPawn :type "Pawn Object Reference"))
  ;[1 1 1] If use actor will move to center of building
  (bind _movementresult (`|AIMoveTo` ControlledPawn (`BTFunctionLibrary.GetBlackboardValueAsVector` (`self.TargetLocation`)) null 500.0 :!label _label)
    (:`OnSuccess`
      (`BTFunctionLibrary.SetBlackboardValueAsObject` (`self.CurrentLocation`) (`BTFunctionLibrary.GetBlackboardValueAsObject` (`self.Destination`)))
      (`BTFunctionLibrary.ClearBlackboardValue` (`self.Destination`))
      (`self.FinishExecute` true))
    (:`OnFail`
      (switch `EPathFollowingResult` _movementresult
        (:`Blocked`
          (goto _label))
        (:`Aborted`
          _)
        (:`Invalid`
          _))
      (`self.FinishExecute` false))))

(event `self.ReceiveAbortAI`
  (params (OwnerController :type "AIController Object Reference") (ControlledPawn :type "Pawn Object Reference"))
  (`Controller.StopMovement` OwnerController)
  (`BTFunctionLibrary.ClearBlackboardValue` (`self.TargetLocation`))
  (`BTFunctionLibrary.ClearBlackboardValue` (`self.Destination`))
  (`BTFunctionLibrary.ClearBlackboardValue` (`self.CurrentLocation`))
  (`self.FinishAbort`))