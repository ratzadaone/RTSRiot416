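; EQS context that supplies pickup/drop-off targets for human units from the buildings in the game state's BuildingQueue.
; ProvideLocationsSet returns each building's Entrance location once per required resource; ProvideActorsSet returns the buildings without duplicates.
; The filter matching the carried pickup to a required resource is disconnected, so every building with requirements qualifies regardless of the querier.
; Both functions print the selected building names as debug output.
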(fn `ProvideActorsSet`
  (params (QuerierObject :type "Object Object Reference") (QuerierActor :type "Actor Object Reference"))
  (returns (ResultingActorsSet :type "Array of Actor Object Reference"))
  (locals (Pawn :type "/Game/Blueprints/Units/BPMasterHumanChar Object Reference") (OneTest :type "/Game/Blueprints/Buildings/BPBuildingMaster Object Reference") (ReturnTests :type "Array of Actor Object Reference"))
  (set `local.Pawn` (cast `/Game/Blueprints/Units/BPMasterHumanChar` QuerierActor :!pure true))
  (for _array_element (`/Game/Blueprints/Game/BPRiotGameState.BuildingQueue` (cast `/Game/Blueprints/Game/BPRiotGameState` (`GameplayStatics.GetGameState`) :!pure true))
    (set `local.OneTest` _array_element)
    (for _array_element_2 (`.BuildingRequiredResources_43_16ECF3C946C5ABD7F8FEC59BAF30D635` (break `/Game/Structs/Building_Properties_Struct` (`/Game/Blueprints/Buildings/BPBuildingMaster.BuildingStructFromTable` _array_element)))
      (`KismetArrayLibrary.Array_AddUnique` (`local.ReturnTests`) (`local.OneTest`))))
  (for _array_element_3 (`local.ReturnTests`)
    (`KismetSystemLibrary.PrintString` (`KismetSystemLibrary.GetObjectName` _array_element_3) true true (struct :`R` 1.0 :`G` 0.225726 :`B` 0.365823 :`A` 1.0) 50.0))
  (return (`local.ReturnTests`)))

(fn `ProvideLocationsSet`
  (params (QuerierObject :type "Object Object Reference") (QuerierActor :type "Actor Object Reference"))
  (returns (ResultingLocationSet :type "Array of Vector Structure"))
  (locals (Pawn :type "/Game/Blueprints/Units/BPMasterHumanChar Object Reference") (OneTest :type "/Game/Blueprints/Buildings/BPBuildingMaster Object Reference") (ReturnLoc :type "Array of Vector Structure") (MultiTest :type "Array of /Game/Blueprints/Buildings/BPBuildingMaster Object Reference"))
  (set `local.Pawn` (cast `/Game/Blueprints/Units/BPMasterHumanChar` QuerierActor :!pure true))
  (for _array_element (`/Game/Blueprints/Game/BPRiotGameState.BuildingQueue` (cast `/Game/Blueprints/Game/BPRiotGameState` (`GameplayStatics.GetGameState`) :!pure true))
    (set `local.OneTest` _array_element)
    (for _array_element_2 (`.BuildingRequiredResources_43_16ECF3C946C5ABD7F8FEC59BAF30D635` (break `/Game/Structs/Building_Properties_Struct` (`/Game/Blueprints/Buildings/BPBuildingMaster.BuildingStructFromTable` _array_element)))
      (`KismetArrayLibrary.Array_Add` (`local.ReturnLoc`) (`SceneComponent.K2_GetComponentLocation` (`/Game/Blueprints/Buildings/BPBuildingMaster.Entrance` (`local.OneTest`))))
      (`KismetArrayLibrary.Array_Add` (`local.MultiTest`) (`local.OneTest`))))
  (for _array_element_3 (`local.MultiTest`)
    (`KismetSystemLibrary.PrintString` (`KismetSystemLibrary.GetObjectName` _array_element_3) true true (struct :`G` 1.0 :`B` 0.029325 :`A` 1.0) 50.0))
  (return (`local.ReturnLoc`)))