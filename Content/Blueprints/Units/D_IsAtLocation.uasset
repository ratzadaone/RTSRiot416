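; Behavior tree decorator that checks whether a human character AI has reached its house or workplace, chosen by LocationCheck.
; It caches the controller and pawn, then compares the CurrentLocation blackboard value to HouseRef for Home, or to the profile's PlaceOfEmployment for the office and factory options.
; Each check writes its result to the pawn's debug info, and a successful workplace check also unpauses the controller's work timer.
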(fn `PerformConditionCheckAI`
  (params (OwnerController :type "AIController Object Reference") (ControlledPawn :type "Pawn Object Reference"))
  (returns (ReturnValue :type Boolean))
  (bind _pawn (`self.Pawn`))
  (bind _returnvalue (== (`BTFunctionLibrary.GetBlackboardValueAsActor` (`self.HouseRef`)) (`BTFunctionLibrary.GetBlackboardValueAsObject` (`self.CurrentLocation`))))
  (bind _returnvalue_2 (== (`BTFunctionLibrary.GetBlackboardValueAsObject` (`self.CurrentLocation`)) (`.PlaceOfEmployment_17_24FB15DC431FF5690B2068901A922B03` (break `/Game/Structs/UnitProperties` (`/Game/Blueprints/Units/BPMasterHumanChar.MyProfile` (`self.Pawn`))))))
  (`/Engine/EditorBlueprintResources/StandardMacros.IsValid` (`self.Controller`)
    (:`Is Valid`
      _)
    (:`Is Not Valid`
      ;[1 1 1] pawnCast
      (set `self.Controller` (cast `/Game/Blueprints/Units/BPAIControllerHumanChar` OwnerController :!pure true))))
  (`/Engine/EditorBlueprintResources/StandardMacros.IsValid` (`self.Pawn`)
    (:`Is Valid`
      _)
    (:`Is Not Valid`
      (set `self.Pawn` (cast `/Game/Blueprints/Units/BPMasterHumanChar` ControlledPawn :!pure true))))
  (switch `/Game/ENums/Enum_LocationType` (`self.LocationCheck`)
    (:`NewEnumerator1`
      ;[1 1 1] Home
      (`/Game/Blueprints/Units/BPMasterHumanChar.SetDebugInfo` _pawn (`KismetStringLibrary.Concat_StrStr` "Check If reached House: " (`KismetStringLibrary.Conv_BoolToString` _returnvalue)))
      (return _returnvalue))
    (:`NewEnumerator2`
      _)
    (:`NewEnumerator5`
      _)
    (:`NewEnumerator10`
      _))
  (`/Game/Blueprints/Units/BPMasterHumanChar.SetDebugInfo` _pawn (`KismetStringLibrary.Concat_StrStr` "Check If reached Office:" (`KismetStringLibrary.Conv_BoolToString` _returnvalue_2)))
  (if _returnvalue_2
    (`KismetSystemLibrary.K2_UnPauseTimerHandle` (`/Game/Blueprints/Units/BPAIControllerHumanChar.WorkHandle` (`self.Controller`))))
  (return _returnvalue_2))