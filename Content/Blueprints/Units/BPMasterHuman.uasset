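; Master Blueprint for human NPC units that randomizes gender, name and body color and highlights on mouse hover.
; The construction script calls RandomFeatures, which creates a dynamic body material, picks a random NPC type and tints BodyColor male or female.
; GetRandomName draws a name from the matching male or female name enum, stored with the type in MyProfile.
; Cursor over the capsule toggles the mesh's custom depth rendering.
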(event `self.CapsuleComponent.OnBeginCursorOver`
  (params (TouchedComponent :type "PrimitiveComponent Object Reference"))
  (`PrimitiveComponent.SetRenderCustomDepth` (`self.Mesh`) true))

(event `self.CapsuleComponent.OnEndCursorOver`
  (params (TouchedComponent :type "PrimitiveComponent Object Reference"))
  (`PrimitiveComponent.SetRenderCustomDepth` (`self.Mesh`) false))

(fn `GetRandomName`
  (params (Type :type "/Game/ENums/Enum_NPCType Enum"))
  (returns (Name :type String))
  (if (`|EnumEquality` Type "NewEnumerator0")
    (return (`|GetEnumeratorNameAsString` (enumliteral `/Game/ENums/Enum_NPCNameMale` (cast `/Game/ENums/Enum_NPCNameMale` (`KismetMathLibrary.Conv_IntToByte` (`KismetMathLibrary.RandomIntegerInRange` 0 (- (enumcount `/Game/ENums/Enum_NPCNameMale`) 1)))))))
    (else
      (return (`|GetEnumeratorNameAsString` (enumliteral `/Game/ENums/Enum_NPCNameFemale` (cast `/Game/ENums/Enum_NPCNameFemale` (`KismetMathLibrary.Conv_IntToByte` (`KismetMathLibrary.RandomIntegerInRange` 0 (- (enumcount `/Game/ENums/Enum_NPCNameFemale`) 1))))))))))

(fn `RandomFeatures`
  (locals (MaterialInstance :type "MaterialInstanceDynamic Object Reference") (FemaleColour :type "LinearColor Structure" :default (struct :`R` 0.7 :`G` 0.240857 :`B` 0.490941)) (MaleColour :type "LinearColor Structure" :default (struct :`R` 0.235679 :`G` 0.18766 :`B` 0.7)))
  (bind _materialinstance (`local.MaterialInstance`))
  (bind _returnvalue (`PrimitiveComponent.CreateDynamicMaterialInstance` (`self.Mesh`) 0 "/Game/Materials/M_UE4Man_Body_Inst.M_UE4Man_Body_Inst"))
  (set `local.MaterialInstance` _returnvalue)
  (if (`|EnumEquality` (enumliteral `/Game/ENums/Enum_NPCType` (cast `/Game/ENums/Enum_NPCType` (`KismetMathLibrary.Conv_IntToByte` (`KismetMathLibrary.RandomIntegerInRange` 0 (- (enumcount `/Game/ENums/Enum_NPCType`) 1))))) "NewEnumerator0")
    (`MaterialInstanceDynamic.SetVectorParameterValue` _materialinstance "BodyColor" (`local.MaleColour`))
    (bind _name (`self.GetRandomName` "NewEnumerator0"))
    (set `self.MyProfile` (make `/Game/Structs/UnitProperties` _name))
    (else
      (`MaterialInstanceDynamic.SetVectorParameterValue` _materialinstance "BodyColor" (`local.FemaleColour`))
      (bind _name_2 (`self.GetRandomName` "NewEnumerator1"))
      (set `self.MyProfile` (make `/Game/Structs/UnitProperties` _name_2 "NewEnumerator1")))))

(fn `UserConstructionScript`
  (`self.RandomFeatures`))