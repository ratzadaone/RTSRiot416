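; EQS context that supplies drop-off targets for a human unit carrying a pickup.
; It scans the game state's building queue and collects, without duplicates, buildings whose required resources match the carried resource's row name.
; Only one pickup type is handled; others print a placeholder message for future tool support.
; A debug print of the matched building's name precedes returning the set.
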(fn `ProvideActorsSet`
  (params (QuerierObject :type "Object Object Reference") (QuerierActor :type "Actor Object Reference"))
  (returns (ResultingActorsSet :type "Array of Actor Object Reference"))
  (locals (ReturnTests :type "Array of Actor Object Reference") (OneTest :type "/Game/Blueprints/Buildings/BPBuildingMaster Object Reference") (Pawn :type "/Game/Blueprints/Units/BPMasterHumanChar Object Reference"))
  (bind _returntests (`local.ReturnTests`))
  (bind (_structpickuptype _structpickupclass _structpickupamount) (break `/Game/Structs/Struct_PickUp` (`/Game/Blueprints/Units/BPMasterHumanChar.UnitPickUpCarryStruct` (`local.Pawn`))))
  (set `local.Pawn` (cast `/Game/Blueprints/Units/BPMasterHumanChar` QuerierActor :!pure true))
  (for _array_element (`/Game/Blueprints/Game/BPRiotGameState.BuildingQueue` (cast `/Game/Blueprints/Game/BPRiotGameState` (`GameplayStatics.GetGameState`) :!pure true))
    (set `local.OneTest` _array_element)
    (for _array_element_2 (`.BuildingRequiredResources_43_16ECF3C946C5ABD7F8FEC59BAF30D635` (break `/Game/Structs/Building_Properties_Struct` (`/Game/Blueprints/Buildings/BPBuildingMaster.BuildingStructFromTable` _array_element)))
      (if (`|EnumEquality` _structpickuptype "NewEnumerator0")
        (if (`|EnumEquality` (`.ResIndex_8_6AB47622472A1F1919F6AB88B36180D9` (break `/Game/Structs/STRUCT_ResourcesIndexes` _array_element_2)) (defaults `/Game/Blueprints/Units/EQ_Context_PickupDropOff` (castclass `/Game/Blueprints/Resources/BPMasterResource` _structpickupclass :!pure true)))
          (`KismetArrayLibrary.Array_AddUnique` (`local.ReturnTests`) (`local.OneTest`)))
        (else
          (`KismetSystemLibrary.PrintString` "add blueprint for tools" true true (struct :`G` 0.66 :`B` 1.0 :`A` 1.0) 20.0)))))
  (for _array_element_3 _returntests
    (`KismetSystemLibrary.PrintString` (`KismetSystemLibrary.GetObjectName` _array_element_3) true true (struct :`G` 1.0 :`B` 0.029325 :`A` 1.0) 50.0)
    (return _returntests))
  (return _returntests))