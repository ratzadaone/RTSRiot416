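; Master resource deposit actor that scatters resource actors inside a configurable box volume at BeginPlay, then registers itself with BPRiotGameState.
; PopulateDeposit reads class, amount and extraction rate from DT_Resources and spawns at seeded random points atop the box until the instance cap or attempt limit.
; Downward traces ground each spawn with Z clamped to the box, adding it to deposit capacity or destroying it on a miss.
; Random rotation and scale nodes are unconnected.
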(event `PopulateDeposit`
  (bind _randomlocationseed (`self.RandomLocationSeed`))
  (bind _spawnareavolume (`self.SpawnAreaVolume`))
  (bind _resourceamount (`self.ResourceAmount`))
  (bind (_returnvalue_x _returnvalue_y _returnvalue_z) (`KismetMathLibrary.BreakVector` (`SceneComponent.K2_GetComponentLocation` _spawnareavolume)))
  (bind (_boxextent_x _boxextent_y _boxextent_z) (`KismetMathLibrary.BreakVector` (`BoxComponent.BoxExtent` _spawnareavolume)))
  (bind (_boxextent_x_2 _boxextent_y_2 _boxextent_z_2) (`KismetMathLibrary.BreakVector` (`BoxComponent.BoxExtent` (`self.SpawnAreaVolume`))))
  ;[1 1 1] Populate Deposit
  (bind _returnvalue (`|GetDataTableRow` "/Game/DataTables/DT_Resources.DT_Resources" (`KismetStringLibrary.Conv_StringToName` (`|GetEnumeratorNameAsString` (enumliteral `/Game/ENums/Enum_ResourcesROwNames` (`self.ResourceName`)))))
    (:`then`
      (bind (_resourceindexenum _resourcemesh _resourcethumbnail _resourceproximitytype _resourceammount _resourceclass _resourceextractionrate) (break `/Game/Structs/Res_Properties_Struct` _returnvalue))
      (set `self.ResourceAmount` (`KismetMathLibrary.Conv_IntToDouble` _resourceammount))
      (for _ (range 1000)
        (if (>= (`self.InstanceCount`) (`self.DepositStartCapacityInstance`))
          (break)
          (else
            (bind _returnvalue_2 (`KismetMathLibrary.ComposeTransforms` (`SceneComponent.K2_GetComponentToWorld` (`self.SpawnAreaVolume`)) (`KismetMathLibrary.MakeTransform` (`KismetMathLibrary.MakeVector` (`KismetMathLibrary.RandomFloatInRangeFromStream` (* _boxextent_x_2 -1.0) _boxextent_x_2 _randomlocationseed) (`KismetMathLibrary.RandomFloatInRangeFromStream` (* _boxextent_y_2 -1.0) _boxextent_y_2 _randomlocationseed) (+ _boxextent_z_2 (`.SphereRadius` (`KismetMathLibrary.BreakBoxSphereBounds` (`StaticMesh.GetBounds` _resourcemesh))))) (struct) (1.0 1.0 1.0))))
            (bind _returnvalue_3 (`|SpawnActorFromClass` _resourceclass _returnvalue_2 "DontSpawnIfColliding" "OverrideRootScale" null self))
            (`/Engine/EditorBlueprintResources/StandardMacros.IsValid` _returnvalue_3
              (:`Is Valid`
                (bind _location (.location _returnvalue_2))
                (bind (_outhit _returnvalue_4) (`KismetSystemLibrary.LineTraceSingle` _location (`KismetMathLibrary.MakeVector` (.x _location) (.y _location) -10000.0) "TraceTypeQuery3"))
                (if _returnvalue_4
                  (`/Engine/EditorBlueprintResources/StandardMacros.IncrementInt` (`self.InstanceCount`)
                    (:`  `
                      (bind (_bblockinghit _binitialoverlap _time _location_2 _impactpoint _normal _impactnormal _physmat _hitactor _hitcomponent _hitbonename _hititem _faceindex _tracestart) (`GameplayStatics.BreakHitResult` _outhit))
                      (bind _returnvalue_location (`KismetMathLibrary.BreakTransform` (`KismetMathLibrary.MakeTransform` (`KismetMathLibrary.MakeVector` (.x _tracestart) (.y _tracestart) (`KismetMathLibrary.FClamp` (.z _impactpoint) (- _returnvalue_z _boxextent_z) (+ _returnvalue_z _boxextent_z))) (struct) (1.0 1.0 1.0))))
                      (`self.K2_SetActorLocation` _returnvalue_3 _returnvalue_location false false)
                      (`KismetArrayLibrary.Array_Add` (`self.ResourceInDeposit`) _returnvalue_3)
                      (set `self.DepositCurrentCapacityAmount` (+ (`self.DepositCurrentCapacityAmount`) (`self.ResourceAmount`)))
                      (set `/Game/Blueprints/Resources/BPMasterResource.ResourceCurrentCarry` _resourceamount _returnvalue_3)
                      (set `/Game/Blueprints/Resources/BPMasterResource.ResourceMaxCarry` _resourceamount _returnvalue_3)
                      (`TextRenderComponent.K2_SetText` (`/Game/Blueprints/Resources/BPMasterResource.TextRender` _returnvalue_3) (`KismetTextLibrary.Conv_DoubleToText` _resourceamount "HalfToEven"))
                      (set `/Game/Blueprints/Resources/BPMasterResource.ResourceExtractionRate` (`KismetMathLibrary.Conv_IntToDouble` _resourceextractionrate) _returnvalue_3)))
                  (else
                    (`self.K2_DestroyActor` _returnvalue_3)))))))))))

(event `self.ReceiveBeginPlay`
  ;[1 1 1] Begin Play
  (`self.PopulateDeposit`)
  (`/Engine/EditorBlueprintResources/StandardMacros.IsValid` (`self.GameStateRef`)
    (:`Is Valid`
      _)
    (:`Is Not Valid`
      (bind _output_get (set `self.GameStateRef` (cast `/Game/Blueprints/Game/BPRiotGameState` (`GameplayStatics.GetGameState`) :!pure true)))))
  (`/Game/Blueprints/Game/BPRiotGameState.AddDepositsToGame` _output_get self (`self.ResourceName`)))

(fn `UserConstructionScript`
  (locals (InstanceIndex_Loc :type Integer) (InstanceAmount :type Integer))
  (`BoxComponent.SetBoxExtent` (`self.SpawnAreaVolume`) (`self.SpawnAreaSize`) true))