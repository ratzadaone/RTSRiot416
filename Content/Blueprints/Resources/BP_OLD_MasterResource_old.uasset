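; Resource node actor, apparently an old master version, that scatters instanced meshes of one resource type inside a box volume.
; The construction script pulls mesh and amount from DT_Resources by ResourceName, then adds instances with seeded random position, rotation and scale.
; Each instance is line-traced downward, height-clamped to the volume, and recorded in ResourceInstances with its amount.
; Hover toggles custom depth on the whole component; click only prints debug text.
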(event `self.InstancedStaticMesh.OnBeginCursorOver`
  (params (TouchedComponent :type "PrimitiveComponent Object Reference"))
  (`PrimitiveComponent.SetRenderCustomDepth` TouchedComponent true))

(event `self.InstancedStaticMesh.OnEndCursorOver`
  (params (TouchedComponent :type "PrimitiveComponent Object Reference"))
  (`PrimitiveComponent.SetRenderCustomDepth` TouchedComponent false))

(event `self.InstancedStaticMesh.OnClicked`
  (params (TouchedComponent :type "PrimitiveComponent Object Reference") (ButtonPressed :type "Key Structure" :default "AnyKey"))
  (`KismetSystemLibrary.PrintString` "Hello"))

(fn `UserConstructionScript`
  (locals (InstanceIndex_Loc :type Integer) (InstanceAmount :type Integer))
  (bind _instancedstaticmesh (`self.InstancedStaticMesh`))
  (bind _randomlocationseed (`self.RandomLocationSeed`))
  (bind _instancedstaticmesh_2 (`self.InstancedStaticMesh`))
  (bind _spawnareavolume (`self.SpawnAreaVolume`))
  (bind (_instanceminscale_x _instanceminscale_y _instanceminscale_z) (`KismetMathLibrary.BreakVector` (`self.InstanceMinScale`)))
  (bind (_instancemaxscale_x _instancemaxscale_y _instancemaxscale_z) (`KismetMathLibrary.BreakVector` (`self.InstanceMaxScale`)))
  (bind _randomsizeseed (`self.RandomSizeSeed`))
  (bind (_returnvalue_x _returnvalue_y _returnvalue_z) (`KismetMathLibrary.BreakVector` (`SceneComponent.K2_GetComponentLocation` _spawnareavolume)))
  (bind _outinstancetransform (`InstancedStaticMeshComponent.GetInstanceTransform` _instancedstaticmesh_2 (`local.InstanceIndex_Loc`) true))
  (bind (_returnvalue_roll _returnvalue_pitch _returnvalue_yaw) (`KismetMathLibrary.BreakRotator` (`KismetMathLibrary.RandomRotatorFromStream` true (`self.RandomRotationSeed`))))
  (bind (_boxextent_x _boxextent_y _boxextent_z) (`KismetMathLibrary.BreakVector` (`BoxComponent.BoxExtent` _spawnareavolume)))
  (bind (_boxextent_x_2 _boxextent_y_2 _boxextent_z_2) (`KismetMathLibrary.BreakVector` (`BoxComponent.BoxExtent` (`self.SpawnAreaVolume`))))
  (bind _returnvalue (`|GetDataTableRow` "/Game/DataTables/DT_Resources.DT_Resources" (`self.ResourceName`))
    (:`then`
      (bind (_resourceindexenum _resourcemesh _resourcethumbnail _resourceproximitytype _resourceammount) (break `/Game/Structs/Res_Properties_Struct` _returnvalue))
      (`StaticMeshComponent.SetStaticMesh` (`self.InstancedStaticMesh`) _resourcemesh)
      (set `local.InstanceAmount` _resourceammount)
      (`BoxComponent.SetBoxExtent` (`self.SpawnAreaVolume`) (`self.SpawnAreaSize`) true)
      (for _ (range 1 (+ (`self.InstanceNr`) 1))
        (bind _returnvalue_2 (`InstancedStaticMeshComponent.AddInstance` _instancedstaticmesh (`KismetMathLibrary.MakeTransform` (`KismetMathLibrary.MakeVector` (`KismetMathLibrary.RandomFloatInRangeFromStream` (* _boxextent_x_2 -1.0) _boxextent_x_2 _randomlocationseed) (`KismetMathLibrary.RandomFloatInRangeFromStream` (* _boxextent_y_2 -1.0) _boxextent_y_2 _randomlocationseed) _boxextent_z_2) (`KismetMathLibrary.MakeRotator` (`KismetMathLibrary.FClamp` _returnvalue_roll 0.0 (`self.RollRotationTreshhold`)) (`KismetMathLibrary.FClamp` _returnvalue_pitch 0.0 (`self.PitchRotationTreshhold`)) (`KismetMathLibrary.FClamp` _returnvalue_yaw 0.0 (`self.YawRotationTreshhold`))) (`KismetMathLibrary.MakeVector` (`KismetMathLibrary.RandomFloatInRangeFromStream` _instanceminscale_x _instancemaxscale_x _randomsizeseed) (`KismetMathLibrary.RandomFloatInRangeFromStream` _instanceminscale_y _instancemaxscale_y _randomsizeseed) (`KismetMathLibrary.RandomFloatInRangeFromStream` _instanceminscale_z _instancemaxscale_z _randomsizeseed)))))
        (set `local.InstanceIndex_Loc` _returnvalue_2)
        (bind _outinstancetransform_2 (`InstancedStaticMeshComponent.GetInstanceTransform` _instancedstaticmesh _returnvalue_2 true))
        (bind _outhit (`KismetSystemLibrary.LineTraceSingle` (.location _outinstancetransform_2) (`KismetMathLibrary.MakeVector` (.x (.location _outinstancetransform_2)) (.y (.location _outinstancetransform_2)) -10000.0) "TraceTypeQuery3"))
        (bind (_bblockinghit _binitialoverlap _time _location _impactpoint _normal _impactnormal _physmat _hitactor _hitcomponent _hitbonename _hititem _faceindex _tracestart) (`GameplayStatics.BreakHitResult` _outhit))
        (bind (_returnvalue_location _returnvalue_rotation _returnvalue_scale) (`KismetMathLibrary.BreakTransform` (`KismetMathLibrary.MakeTransform` (`KismetMathLibrary.MakeVector` (.x _tracestart) (.y _tracestart) (`KismetMathLibrary.FClamp` (.z _impactpoint) (- _returnvalue_z _boxextent_z) (+ _returnvalue_z _boxextent_z))) (.rotation _outinstancetransform) (.scale _outinstancetransform))))
        (`InstancedStaticMeshComponent.UpdateInstanceTransform` _instancedstaticmesh_2 (`local.InstanceIndex_Loc`) (`KismetMathLibrary.MakeTransform` _returnvalue_location _returnvalue_rotation _returnvalue_scale) true false false)
        (`BlueprintMapLibrary.Map_Add` (`self.ResourceInstances`) _returnvalue_location (`local.InstanceAmount`))))))