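; Day-night controller that rotates the sun and moon lights to follow the game state's time of day.
; On BeginPlay, the SunMovement timeline starts from the game state's Hours at a play rate inversely proportional to TimeUnit.
; Each timeline update applies pitch and yaw tracks to both lights, then refreshes the sky sphere's sun direction.
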(event `self.ReceiveBeginPlay`
  (bind _asbpriot_game_state (cast `/Game/Blueprints/Game/BPRiotGameState` (`GameplayStatics.GetGameState`) :!pure true))
  (`self.SetNewTime`)
  (`TimelineComponent.SetPlayRate` (`self.SunMovement`) (/ 1.0 (`/Game/Blueprints/Game/BPRiotGameState.TimeUnit` _asbpriot_game_state)))
  (bind (_direction _sunpitch _sunyaw _moonpitch _moonyaw) (`Timeline|SunMovement` :`NewTime` (`KismetMathLibrary.Conv_IntToDouble` (`/Game/Blueprints/Game/BPRiotGameState.Hours` _asbpriot_game_state)) :!label _label)
    (:`Update`
      (`self.K2_SetActorRotation` (`self.LightSource`) (`KismetMathLibrary.MakeRotator` 0.0 _sunpitch _sunyaw) false)
      (`self.K2_SetActorRotation` (`self.MoonLight`) (`KismetMathLibrary.MakeRotator` 0.0 _moonpitch _moonyaw) false)
      (`/Game/Sky/BP_Sky_Sphere_MOD.UpdateSunDirection` (`self.SkySphere`)))))

(event `SetNewTime`
  (goto _label :!via `SetNewTime`))

(fn `UserConstructionScript`)