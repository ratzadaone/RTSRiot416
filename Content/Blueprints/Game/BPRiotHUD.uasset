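; BPRiotHUD is a HUD that draws the drag-selection box for human units.
; On BeginPlay it caches the owning riot pawn and the player controller.
; While IsDrawing is set, DrawHUD stretches a translucent texture from ClickedLocation to the mouse cursor.
; It then passes every BPUnitHuman inside that rectangle to the controller's PreselectedUnits via GetActorsInSelectionRectangle.
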(event `self.ReceiveBeginPlay`
  (bind _asbpriot_pawn (cast `/Game/Blueprints/Player/BPRiotPawn` (`self.GetOwningPawn`))
    (:`then`
      (set `self.PawnRef` _asbpriot_pawn)
      (bind _asbpriot_controller (cast `/Game/Blueprints/Player/BPRiotController` (`GameplayStatics.GetPlayerController` 0))
        (:`then`
          (set `self.ControllerRef` _asbpriot_controller))
        (:`CastFailed`
          (`KismetSystemLibrary.PrintString` "cast to controller failed"))))
    (:`CastFailed`
      (`KismetSystemLibrary.PrintString` "Cast to Pawn Failed"))))

(event `self.ReceiveDrawHUD`
  (params (SizeX :type Integer) (SizeY :type Integer))
  (bind _clickedlocation (`self.ClickedLocation`))
  (bind (_locationx _locationy) (`PlayerController.GetMousePosition` (`self.ControllerRef`)))
  (bind (_x _y) (`KismetMathLibrary.BreakVector2D` _clickedlocation))
  (bind (_x_2 _y_2) (`KismetMathLibrary.BreakVector2D` (- (`self.CurrentLocation`) _clickedlocation)))
  (set `self.ScreenRes` (`KismetMathLibrary.MakeVector2D` (`KismetMathLibrary.Conv_IntToDouble` SizeX) (`KismetMathLibrary.Conv_IntToDouble` SizeY)))
  (if (`self.IsDrawing`)
    (set `self.CurrentLocation` (`KismetMathLibrary.MakeVector2D` _locationx _locationy))
    (`self.DrawTexture` "/Game/Textures/T_Button_BG_16x16.T_Button_BG_16x16" _x _y _x_2 _y_2 0.0 0.0 0.0 0.0 (struct :`R` 1.0 :`G` 1.0 :`B` 1.0 :`A` 0.159))
    (set `/Game/Blueprints/Player/BPRiotController.PreselectedUnits` (`self.GetActorsInSelectionRectangle` "/Game/Blueprints/Units/BPUnitHuman.BPUnitHuman_C" (`self.ClickedLocation`) (`self.CurrentLocation`)) (`self.ControllerRef`))))

(fn `UserConstructionScript`)