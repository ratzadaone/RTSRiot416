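; Blueprint function library with a helper that sizes and places a box collision against a building mesh.
; The box takes its depth and height from CollisionBoxDistance and CollisionBoxHeight, and its Y extent from the mesh's local minimum bound, slightly inset.
; It is offset along +X by the absolute minimum X bound plus its depth, and raised so its bottom sits at the parent's origin.
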(fn `SetBuildingColisionBox`
  (params (Collision :type "BoxComponent Object Reference") (Mesh :type "StaticMeshComponent Object Reference"))
  (locals (CollisionBoxDistance :type "Float (double-precision)" :default 50.0) (CollisionBoxHeight :type "Float (double-precision)" :default 20.0))
  (bind _min (`StaticMeshComponent.GetLocalBounds` Mesh))
  (`BoxComponent.SetBoxExtent` Collision (`KismetMathLibrary.MakeVector` (`local.CollisionBoxDistance`) (- (`KismetMathLibrary.Abs` (.y _min)) 10.0) (`local.CollisionBoxHeight`)) true)
  (`SceneComponent.K2_SetRelativeLocation` Collision (`KismetMathLibrary.MakeVector` (+ (`KismetMathLibrary.Abs` (.x _min)) (`local.CollisionBoxDistance`)) 0.0 (`local.CollisionBoxHeight`)) false false)
  (return))