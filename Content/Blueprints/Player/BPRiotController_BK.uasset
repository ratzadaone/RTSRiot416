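; Player controller for the Riot game that drives an RTS-style camera on BPRiotPawn.
; BeginPlay caches pawn, game state and HUD references, shows the cursor and spawns widgets from WidgetList.
; Axis input moves the pawn at a speed scaled by spring arm length, while mouse events drive screen-edge scrolling.
; Holding Pan opens gates for mouse rotation with clamped pitch and suspends edge scrolling; zoom inputs adjust arm length within limits.
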(event `self.ReceiveBeginPlay`
  (bind _widgetlist_widgetindex (break `/Game/Structs/WidgetIndexes` (`self.WidgetList`)))
  ;[1 1 1] Begin Play
  (`|ExecutionSequence`
    (:`then_0`
      (bind _asbpriot_pawn (cast `/Game/Blueprints/Player/BPRiotPawn` (`GameplayStatics.GetPlayerPawn` 0))
        (:`then`
          (set `self.PlayerPawnRef` _asbpriot_pawn)
          (bind _asbpriot_game_state (cast `/Game/Blueprints/Player/BPRiotGameState` (`GameplayStatics.GetGameState`))
            (:`then`
              (set `self.GameStateRef` _asbpriot_game_state)
              (bind _asbpriot_hud (cast `/Game/Blueprints/Player/BPRiotHUD` (`self.GetHUD`))
                (:`then`
                  (set `self.HUDRef` _asbpriot_hud))
                (:`CastFailed`
                  (`KismetSystemLibrary.PrintString` "Cast to HUD failed"))))
            (:`CastFailed`
              (`KismetSystemLibrary.PrintString` "Cast Game state failed"))))
        (:`CastFailed`
          (`KismetSystemLibrary.PrintString` "CastFailed"))))
    (:`then_1`
      (`WidgetBlueprintLibrary.SetInputMode_GameAndUIEx` self null "DoNotLock" false)
      (set `self.bShowMouseCursor` true))
    (:`then_2`
      (for _array_element _widgetlist_widgetindex
        (bind _returnvalue (`|CreateWidget` (break `/Game/Structs/WIdgetProperies` _array_element)))
        (`UserWidget.AddToViewport` _returnvalue 0)
        (`Widget.SetVisibility` _returnvalue "Visible")))))

(event `InputAxis|MoveForward`
  (params (AxisValue :type "Float (single-precision)"))
  (bind _playerpawnref (`self.PlayerPawnRef`))
  (bind _returnvalue (`self.GetTransform` _playerpawnref))
  ;[1 1 1] Keyboardcamera Controls
  (if (not (`self.bDisableCamNav`))
    (`self.K2_SetActorTransform` (`self.PlayerPawnRef`) (`KismetMathLibrary.MakeTransform` (+ (`KismetMathLibrary.TransformDirection` _returnvalue (`KismetMathLibrary.MakeVector` (* (* AxisValue (`KismetMathLibrary.FClamp` (/ (`SpringArmComponent.TargetArmLength` (`/Game/Blueprints/Player/BPRiotPawn.SpringArm` _playerpawnref)) 100.0) 5.0 20.0)) (`self.FastMoveMultiplier`)))) (.location _returnvalue)) (.rotation _returnvalue) (.scale _returnvalue)) false false)))

(event `InputAxis|MoveRight`
  (params (AxisValue :type "Float (single-precision)"))
  (bind _playerpawnref (`self.PlayerPawnRef`))
  (bind _returnvalue (`self.GetTransform` _playerpawnref))
  ;[1 1 1] Keyboardcamera Controls
  (`self.K2_SetActorTransform` (`self.PlayerPawnRef`) (`KismetMathLibrary.MakeTransform` (+ (`KismetMathLibrary.TransformDirection` _returnvalue (`KismetMathLibrary.MakeVector` 0.0 (* (* (`KismetMathLibrary.FClamp` (/ (`SpringArmComponent.TargetArmLength` (`/Game/Blueprints/Player/BPRiotPawn.SpringArm` _playerpawnref)) 100.0) 5.0 20.0) (`self.FastMoveMultiplier`)) AxisValue))) (.location _returnvalue)) (.rotation _returnvalue) (.scale _returnvalue)) false false))

(event `InputAxisKey|MouseX`
  (params (AxisValue :type "Float (single-precision)"))
  (bind (_returnvalue_roll _returnvalue_pitch _returnvalue_yaw) (`KismetMathLibrary.BreakRotator` (`self.K2_GetActorRotation` (`self.PlayerPawnRef`))))
  ;[1 1 1] Pan X and Y
  (`|ExecutionSequence`
    (:`then_0`
      (`self.PanX`))
    (:`then_1`
      (`/Engine/EditorBlueprintResources/StandardMacros.Gate` true :!label _label
        (:`Exit`
          (`self.K2_SetActorRotation` (`self.PlayerPawnRef`) (`KismetMathLibrary.MakeRotator` _returnvalue_roll _returnvalue_pitch (+ _returnvalue_yaw (* AxisValue (`self.PanSensitivity`)))) false))))))

(event `InputAction|Pan`
  (params (Key :type "Key Structure" :default "AnyKey"))
  ;[1 1 1] Pan X and Y
  (:`Pressed`
    (set `self.bDisableCamNav` true)
    (goto _label :!via `Open`))
  (:`Released`
    (set `self.bDisableCamNav` false)
    (goto _label :!via `Close`)))

(event `InputAxisKey|MouseY`
  (params (AxisValue :type "Float (single-precision)"))
  (bind (_returnvalue_roll _returnvalue_pitch _returnvalue_yaw) (`KismetMathLibrary.BreakRotator` (`self.K2_GetActorRotation` (`self.PlayerPawnRef`))))
  ;[1 1 1] Pan X and Y
  (`|ExecutionSequence`
    (:`then_0`
      (`self.PanY`))
    (:`then_1`
      (`/Engine/EditorBlueprintResources/StandardMacros.Gate` true :!label _label_2
        (:`Exit`
          (`self.K2_SetActorRotation` (`self.PlayerPawnRef`) (`KismetMathLibrary.MakeRotator` _returnvalue_roll (`KismetMathLibrary.FClamp` (+ _returnvalue_pitch (* AxisValue (`self.PanSensitivity`))) -15.0 45.0) _returnvalue_yaw) false))))))

(event `InputAction|Pan`
  (params (Key :type "Key Structure" :default "AnyKey"))
  ;[1 1 1] Pan X and Y
  (:`Pressed`
    (set `self.bDisableCamNav` true)
    (goto _label_2 :!via `Open`))
  (:`Released`
    (set `self.bDisableCamNav` false)
    (goto _label_2 :!via `Close`)))

(event `PanX`
  (bind (_returnvalue_x _returnvalue_y) (`KismetMathLibrary.BreakVector2D` (`WidgetLayoutLibrary.GetViewportSize`)))
  (bind _fastmovemultiplier (`self.FastMoveMultiplier`))
  (bind _returnvalue (/ (`self.GetMousePosition`) _returnvalue_x))
  ;[1 1 1] Screen Edge Movement
  (if (not (`self.bDisableCamNav`))
    (if (>= _returnvalue 0.975)
      (set `self.EdgeMovementSpeedX` 5.0)
      (elif (<= _returnvalue 0.025)
        (set `self.EdgeMovementSpeedX` -5.0)
        (else
          (set `self.EdgeMovementSpeedX` 0.0))))
    (`self.K2_AddActorLocalOffset` (`self.PlayerPawnRef`) (`KismetMathLibrary.MakeVector` (* (`self.EdgeMovementSpeedY`) _fastmovemultiplier) (* _fastmovemultiplier (`self.EdgeMovementSpeedX`))) false false :!label _label_3)))

(event `PanY`
  (bind (_returnvalue_x _returnvalue_y) (`KismetMathLibrary.BreakVector2D` (`WidgetLayoutLibrary.GetViewportSize`)))
  (bind _returnvalue (/ (`.LocationY` (`self.GetMousePosition`)) _returnvalue_y))
  ;[1 1 1] Screen Edge Movement
  (if (`self.bDisableCamNav`)
    _
    (elif (>= _returnvalue 0.975)
      (set `self.EdgeMovementSpeedY` -5.0)
      (goto _label_3)
      (elif (<= _returnvalue 0.025)
        (set `self.EdgeMovementSpeedY` 5.0)
        (goto _label_3)
        (else
          (set `self.EdgeMovementSpeedY` 0.0)
          (goto _label_3))))))

(event `InputAction|ZoomIn`
  (params (Key :type "Key Structure" :default "AnyKey"))
  (bind _springarm (`/Game/Blueprints/Player/BPRiotPawn.SpringArm` (`self.PlayerPawnRef`)))
  ;[1 1 1] Zoom
  (:`Pressed`
    (set `SpringArmComponent.TargetArmLength` (`KismetMathLibrary.FClamp` (- (`SpringArmComponent.TargetArmLength` _springarm) (`self.ZoomSensitivity`)) (`self.MinZoomDistance`) (`self.MaxArmDistance`)) _springarm)))

(event `InputAction|ZoomOut`
  (params (Key :type "Key Structure" :default "AnyKey"))
  (bind _springarm (`/Game/Blueprints/Player/BPRiotPawn.SpringArm` (`self.PlayerPawnRef`)))
  ;[1 1 1] Zoom
  (:`Pressed`
    (set `SpringArmComponent.TargetArmLength` (`KismetMathLibrary.FClamp` (+ (`self.ZoomSensitivity`) (`SpringArmComponent.TargetArmLength` _springarm)) (`self.MinZoomDistance`) (`self.MaxArmDistance`)) _springarm)))

(fn `UserConstructionScript`)