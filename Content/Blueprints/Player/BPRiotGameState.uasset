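; Game state Blueprint that runs an in-game clock and calendar.
; Each tick, SetClockwork advances a fractional-hour counter by delta seconds over TimeUnit, wrapping at 24 and yielding a day increment.
; Clock converts that counter into the seconds, minutes and hours stored in GameTime.
; Calendar adds the day increment, rolls over months and years using DaysInMonth, and stores GameDate.
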(event `self.ReceiveBeginPlay`
  (set `self.Clockwork` (+ (`KismetMathLibrary.Conv_IntToDouble` (`self.Hours`)) (`KismetMathLibrary.Conv_IntToDouble` (`self.Minutes`)) (`KismetMathLibrary.Conv_IntToDouble` (`self.Hours`))))
  (set `self.GameDate` (`|MakeArray` (`self.Day`) (`self.Month`) (`self.Year`))))

(event `self.ReceiveTick`
  (params (DeltaSeconds :type "Float (single-precision)"))
  (bind (_clockwork _daytick) (`self.SetClockwork` DeltaSeconds (`self.TimeUnit`) (`self.Clockwork`)))
  (set `self.Clockwork` _clockwork)
  (set `self.DayTick` _daytick)
  (`self.Clock`)
  (`self.Calendar`))

(fn `Calendar`
  (bind _output_get (set `self.Day` (+ (`self.Day`) (`self.DayTick`))))
  (if (> _output_get (`KismetMathLibrary.DaysInMonth` (`self.Year`) (`self.Month`)))
    (set `self.Day` 1)
    (set `self.Month` (+ (`self.Month`) 1)))
  (if (> (`self.Month`) 12)
    (set `self.Month` 1)
    (set `self.Year` (+ (`self.Year`) 1)))
  (set `self.GameDate` (`|MakeArray` (`self.Day`) (`self.Month`) (`self.Year`))))

(fn `Clock`
  (bind (_remainder _returnvalue) (`KismetMathLibrary.FMod` (* (`self.Clockwork`) 3600.0) 60.0))
  (bind (_remainder_2 _returnvalue_2) (`KismetMathLibrary.FMod` (`KismetMathLibrary.Conv_IntToDouble` _returnvalue) 60.0))
  (set `self.Seconds` (`KismetMathLibrary.FFloor` _remainder))
  (set `self.Minutes` (`KismetMathLibrary.FFloor` _remainder_2))
  (set `self.Hours` (`KismetMathLibrary.FFloor` (`KismetMathLibrary.FMod` (`KismetMathLibrary.Conv_IntToDouble` _returnvalue_2) 24.0)))
  (set `self.GameTime` (`|MakeArray` (`self.Seconds`) (`self.Minutes`) (`self.Hours`))))

(fn `SetClockwork`
  (params (DeltaSeconds :type "Float (double-precision)") (TimeUnit :type "Float (double-precision)") (ClockworkIn :type "Float (double-precision)"))
  (returns (Clockwork :type "Float (double-precision)") (DayTick :type Integer))
  (bind (_remainder _returnvalue) (`KismetMathLibrary.FMod` (+ (/ DeltaSeconds TimeUnit) ClockworkIn) 24.0))
  (return _remainder _returnvalue))

(fn `UserConstructionScript`)