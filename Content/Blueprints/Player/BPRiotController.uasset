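; Player controller for an RTS-style builder, handling camera navigation, mouse selection and spline road placement.
; Input moves, pans and zooms the spring-arm pawn, with zoom-scaled speed and screen-edge scrolling.
; Tick traces under the cursor to update the road preview, which clicks commit as chained segments continuing the previous tangent.
; A gated looping timer separates clicks from HUD selection-box drags; selection and building mode are stubs.
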(event `self.ReceiveBeginPlay`
  (bind _widgetlist_widgetindex (break `/Game/Structs/WidgetIndexes` (`self.WidgetList`)))
  ;[1 1 1] Begin Play
  (`|ExecutionSequence`
    (:`then_0`
      (bind _asbpriot_pawn (cast `/Game/Blueprints/Player/BPRiotPawn` (`GameplayStatics.GetPlayerPawn` 0))
        (:`then`
          (set `self.PlayerPawnRef` _asbpriot_pawn)
          (bind _asbpriot_game_state (cast `/Game/Blueprints/Game/BPRiotGameState` (`GameplayStatics.GetGameState`))
            (:`then`
              (set `self.GameStateRef` _asbpriot_game_state)
              (bind _asbpriot_hud (cast `/Game/Blueprints/Game/BPRiotHUD` (`self.GetHUD`))
                (:`then`
                  (set `self.GameHUDRef` _asbpriot_hud)
                  ;;[1 1 1] Initialize timed event
                  (`self.CheckForSelection`))
                (:`CastFailed`
                  (`KismetSystemLibrary.PrintString` "gameHUD cast failed"))))
            (:`CastFailed`
              (`KismetSystemLibrary.PrintString` "Cast Game state failed"))))
        (:`CastFailed`
          (`KismetSystemLibrary.PrintString` "CastFailed"))))
    (:`then_1`
      (`WidgetBlueprintLibrary.SetInputMode_GameAndUIEx` self null "DoNotLock" false)
      (set `self.bShowMouseCursor` true))
    (:`then_2`
      (for (_array_element _array_index) _widgetlist_widgetindex
        (bind _returnvalue (`|CreateWidget` (break `/Game/Structs/WIdgetProperies` _array_element)))
        (`UserWidget.AddToViewport` _returnvalue 0)
        (`Widget.SetVisibility` _returnvalue (`.WidgetVisibility_6_5F7113ED4EFF8D9F89778ABCE8B2D9D7` (break `/Game/Structs/WIdgetProperies` _array_element)))
        ;;[1 0.05203 0.2424] HARDCODED Have TO FIX
        (if (== _array_index 0)
          (set `self.WidgetHUDRef` (cast `/Game/Blueprints/Widgets/WMainUI` _returnvalue :!pure true)))))))

(event `InputAxis|MoveForward`
  (params (AxisValue :type "Float (single-precision)"))
  ;[1 1 1] CameraMovement
  ;;[1 1 1] Movement X
  (if (not (`self.bDisableCamNav`))
    (`self.K2_SetActorTransform` (`self.PlayerPawnRef`) (`self.MovementX` (`self.MovementSpeedCalc`) (`self.FastMoveMultiplier`) AxisValue (`self.PlayerPawnRef`)) false false)))

(event `InputAxis|MoveRight`
  (params (AxisValue :type "Float (single-precision)"))
  (bind (_transform_location _transform_rotation _transform_scale) (`KismetMathLibrary.BreakTransform` (`self.MovementY` AxisValue (`self.MovementSpeedCalc`) (`self.FastMoveMultiplier`) (`self.PlayerPawnRef`))))
  ;[1 1 1] CameraMovement
  ;;[1 1 1] MovementY
  (if (not (`self.bDisableCamNav`))
    (`self.K2_SetActorTransform` (`self.PlayerPawnRef`) (`KismetMathLibrary.MakeTransform` (`KismetMathLibrary.MakeVector` (.x _transform_location) (.y _transform_location) (`self.CameraDefaultHeight`)) _transform_rotation _transform_scale) false false)))

(event `InputAxisKey|MouseX`
  (params (AxisValue :type "Float (single-precision)"))
  ;[1 1 1] CameraMovement
  ;;[1 1 1] Pan X
  (`|ExecutionSequence`
    (:`then_0`
      (`/Engine/EditorBlueprintResources/StandardMacros.Gate` true :!label _label
        (:`Exit`
          (`self.K2_SetActorRotation` (`self.PlayerPawnRef`) (`KismetMathLibrary.MakeRotator` (.roll (`self.K2_GetActorRotation` (`self.PlayerPawnRef`))) (.pitch (`self.K2_GetActorRotation` (`self.PlayerPawnRef`))) (+ (.yaw (`self.K2_GetActorRotation` (`self.PlayerPawnRef`))) (* (`self.PanSensitivity`) AxisValue))) false))))
    (:`then_1`
      ;;[1 1 1] EdgeMovement
      (if (not (`self.bDisableCamNav`))
        (bind (_deltaxspeed _deltayspeed) (`self.ScreenEdgeMovement` :!label _label_2)
          (:`NewParam`
            (`self.K2_AddActorLocalOffset` (`self.PlayerPawnRef`) (`KismetMathLibrary.MakeVector` _deltayspeed _deltaxspeed) false false)))))))

(event `InputAction|PanReset`
  (params (Key :type "Key Structure" :default "AnyKey"))
  (bind _playerpawnref (`self.PlayerPawnRef`))
  (bind (_returnvalue_roll _returnvalue_pitch _returnvalue_yaw) (`KismetMathLibrary.BreakRotator` (`self.K2_GetActorRotation` _playerpawnref)))
  ;[1 1 1] CameraMovement
  ;;[1 1 1] Pan Reset - ALT + Middle
  (:`Pressed`
    (`self.K2_SetActorRotation` _playerpawnref (`KismetMathLibrary.MakeRotator` _returnvalue_roll 0.0 _returnvalue_yaw) false)))

(event `InputAction|Pan`
  (params (Key :type "Key Structure" :default "AnyKey"))
  ;[1 1 1] CameraMovement
  ;;[1 1 1] Pan X
  (:`Pressed`
    (set `self.bDisableCamNav` true)
    (goto _label :!via `Open`))
  (:`Released`
    (set `self.bDisableCamNav` false)
    (goto _label :!via `Close`)))

(event `InputAction|ZoomReset`
  (params (Key :type "Key Structure" :default "AnyKey"))
  ;[1 1 1] CameraMovement
  ;;[1 1 1] Zoom Reset
  (:`Pressed`
    (set `SpringArmComponent.TargetArmLength` (`self.DefaultArmDistance`) (`/Game/Blueprints/Player/BPRiotPawn.SpringArm` (`self.PlayerPawnRef`)))))

(event `Key|LeftShift`
  (params (Key :type "Key Structure" :default "AnyKey"))
  ;[1 1 1] CameraMovement
  ;;[1 1 1] Fast Move Multiplier - SHIFT
  (:`Pressed`
    (set `self.FastMoveMultiplier` 2.0))
  (:`Released`
    (set `self.FastMoveMultiplier` 1.0)))

(event `InputAxisKey|MouseY`
  (params (AxisValue :type "Float (single-precision)"))
  ;[1 1 1] CameraMovement
  ;;[1 1 1] Pan Y
  (`|ExecutionSequence`
    (:`then_0`
      (`/Engine/EditorBlueprintResources/StandardMacros.Gate` true :!label _label_3
        (:`Exit`
          (`self.K2_SetActorRotation` (`self.PlayerPawnRef`) (`KismetMathLibrary.MakeRotator` (.roll (`self.K2_GetActorRotation` (`self.PlayerPawnRef`))) (`KismetMathLibrary.FClamp` (+ (.pitch (`self.K2_GetActorRotation` (`self.PlayerPawnRef`))) (* (`self.PanSensitivity`) AxisValue)) -15.0 45.0) (.yaw (`self.K2_GetActorRotation` (`self.PlayerPawnRef`)))) false))))
    (:`then_1`
      ;;[1 1 1] EdgeMovement
      (if (not (`self.bDisableCamNav`))
        (goto _label_2 :!via `MouseY`)))))

(event `InputAction|Pan`
  (params (Key :type "Key Structure" :default "AnyKey"))
  ;[1 1 1] CameraMovement
  ;;[1 1 1] Pan Y
  (:`Pressed`
    (set `self.bDisableCamNav` true)
    (goto _label_3 :!via `Open`))
  (:`Released`
    (set `self.bDisableCamNav` false)
    (goto _label_3 :!via `Close`)))

(event `InputAction|ZoomIn`
  (params (Key :type "Key Structure" :default "AnyKey"))
  (bind _springarm (`/Game/Blueprints/Player/BPRiotPawn.SpringArm` (`self.PlayerPawnRef`)))
  ;[1 1 1] CameraMovement
  ;;[1 1 1] Zoom IN Out MouseWHEEL
  (:`Pressed`
    (set `SpringArmComponent.TargetArmLength` (`KismetMathLibrary.FClamp` (- (`SpringArmComponent.TargetArmLength` _springarm) (`self.ZoomSensitivity`)) (`self.MinZoomDistance`) (`self.MaxArmDistance`)) _springarm)))

(event `InputAction|ZoomOut`
  (params (Key :type "Key Structure" :default "AnyKey"))
  (bind _springarm (`/Game/Blueprints/Player/BPRiotPawn.SpringArm` (`self.PlayerPawnRef`)))
  ;[1 1 1] CameraMovement
  ;;[1 1 1] Zoom IN Out MouseWHEEL
  (:`Pressed`
    (set `SpringArmComponent.TargetArmLength` (`KismetMathLibrary.FClamp` (+ (`SpringArmComponent.TargetArmLength` _springarm) (`self.ZoomSensitivity`)) (`self.MinZoomDistance`) (`self.MaxArmDistance`)) _springarm)))

(event `self.ReceiveTick`
  (params (DeltaSeconds :type "Float (single-precision)"))
  (bind _output_get (set `self.HoverHitResult` (`self.GetHitResultUnderCursorByChannel` "TraceTypeQuery1" false)))
  (if (`|EnumEquality` (`self.GameMode`) "NewEnumerator1")
    (`self.UpdateRoad` (`KismetMathLibrary.MakeTransform` (`.Location` (`GameplayStatics.BreakHitResult` _output_get)) (`KismetMathLibrary.ComposeRotators` (`KismetMathLibrary.MakeRotFromZ` (`.Normal` (`GameplayStatics.BreakHitResult` _output_get))) (`KismetMathLibrary.RotatorFromAxisAndAngle` (`.Normal` (`GameplayStatics.BreakHitResult` _output_get)) (`self.PlacementRotation`)))))))

(event `SpawnRoadPreview`
  (bind _preview (`self.Preview`))
  (set `self.GameMode` "NewEnumerator1")
  (`self.DeselectAll`)
  (if (`KismetSystemLibrary.IsValid` _preview)
    (`self.K2_DestroyActor` _preview))
  (bind _returnvalue (`|SpawnActorFromClass` "/Game/Blueprints/Preview/BPRoadPreview.BPRoadPreview_C" (`KismetMathLibrary.MakeTransform` (0.0 0.0 0.0)) "AlwaysSpawn" "OverrideRootScale"))
  (set `self.Preview` _returnvalue)
  (set `self.RoadMode` 0)
  (`KismetSystemLibrary.PrintString` "HelloRoad"))

(event `SpawnBuildingPreview`
  (params (BuildingClass :type "/Game/Blueprints/Buildings/BPMasterBuilding Class Reference"))
  (set `self.GameMode` "NewEnumerator0"))

(event `UpdateRoad`
  (params (Transform :type "Transform Structure"))
  (bind _location (.location Transform))
  (switch `int` (`self.RoadMode`)
    (:`0`
      (`KismetSystemLibrary.DrawDebugSphere` _location 50.0 12 (struct :`R` 1.0 :`G` 0.008376 :`A` 1.0) 0.1 5.0))
    (:`1`
      (bind _asbproad_preview (cast `/Game/Blueprints/Preview/BPRoadPreview` (`self.Preview`))
        (:`then`
          (`/Game/Blueprints/Preview/BPRoadPreview.SetMidPoint` _asbproad_preview _location true)
          (if (`self.BuildingEnabled`) :!label _label
            (bind _roadspline (`/Game/Blueprints/Preview/BPRoadPreview.RoadSpline` _asbproad_preview))
            (bind _midpoint (`/Game/Blueprints/Preview/BPRoadPreview.MidPoint` _asbproad_preview))
            ;[1 1 1] DEbug Lines
            (`KismetSystemLibrary.DrawDebugLine` (`SplineMeshComponent.GetStartPosition` _roadspline) _midpoint (struct :`R` 0.9 :`G` 0.212102 :`B` 0.412134 :`A` 1.0))
            (`KismetSystemLibrary.DrawDebugLine` (`SplineMeshComponent.GetEndPosition` _roadspline) _midpoint (struct :`R` 0.174199 :`G` 0.220356 :`B` 0.885 :`A` 1.0))))
        (:`CastFailed`
          (`KismetSystemLibrary.PrintString` "Fail Cast To Road Preview"))))
    (:`2`
      (`/Game/Blueprints/Preview/BPRoadPreview.SetEndPoint` _asbproad_preview _location)
      (goto _label))))

(event `CreateRoad`
  (bind _returnvalue (`|SpawnActorFromClass` "/Game/Blueprints/Buildings/BPRoad.BPRoad_C" (`KismetMathLibrary.MakeTransform` (0.0 0.0 0.0)) "AlwaysSpawn" "OverrideRootScale"))
  (`/Game/Blueprints/Buildings/BPRoad.Create` _returnvalue "")
  (`KismetArrayLibrary.Array_Add` (`self.Roads`) _returnvalue))

(event `AppendRoad`
  (params (Road :type "/Game/Blueprints/Buildings/BPRoad Object Reference") (StartPosition :type "Vector Structure") (StartTangent :type "Vector Structure") (EndPosition :type "Vector Structure") (EndTangent :type "Vector Structure"))
  (`/Game/Blueprints/Buildings/BPRoad.AddSpline` Road StartPosition StartTangent EndPosition EndTangent))

(event `FinishRoad`
  (set `self.GameMode` "NewEnumerator3")
  (`self.K2_DestroyActor` (`self.Preview`)))

(event `DeselectAll`
  ;[1 1 1] 2DO
  (`KismetSystemLibrary.PrintString` "Deselect All"))

(event `InputAction|PlaceOrSelect`
  (params (Key :type "Key Structure" :default "AnyKey"))
  ;[1 1 1] LeftClick for Select Place
  (:`Pressed`
    (`self.PlaceSelectPressed`))
  (:`Released`
    (`self.PlaceSelectReleased`)))

(event `CheckForSelection`
  ;[1 1 1] TimerToCheck for Selection Box
  (`KismetSystemLibrary.K2_SetTimerDelegate` (delegate `RunTheGate`) 0.075 true))

(event `RunTheGate`
  (bind (_locationx _locationy) (`self.GetMousePosition`))
  (bind (_hoverhitresult_bblockinghit _hoverhitresult_binitialoverlap _hoverhitresult_time _hoverhitresult_location) (`GameplayStatics.BreakHitResult` (`self.HoverHitResult`)))
  (bind (_clickedlocation_x _clickedlocation_y) (`KismetMathLibrary.BreakVector2D` (`self.ClickedLocation`)))
  (bind _gamehudref (`self.GameHUDRef`))
  ;[1 1 1] TimerToCheck for Selection Box
  (`/Engine/EditorBlueprintResources/StandardMacros.Gate` true :!label _label
    (:`Exit`
      (if (and (== _clickedlocation_x _locationx) (== _clickedlocation_y _locationy))
        ;[1 1 1] NOT selection BOX
        (set `/Game/Blueprints/Game/BPRiotHUD.IsDrawing` false _gamehudref)
        (set `self.SingleClick` true)
        (switch `/Game/ENums/Enum_GameMode` (`self.GameMode`)
          (:`NewEnumerator0`
            (`KismetSystemLibrary.PrintString` "Building Mode"))
          (:`NewEnumerator1`
            ;[1 1 1] New Road so far
            (bind _success (`self.PlaceNewBuilding` _hoverhitresult_location))
            (if _success
              _)))
        (else
          ;[1 1 1] Draw Selection BOX
          (set `/Game/Blueprints/Game/BPRiotHUD.IsDrawing` true _gamehudref)
          (set `/Game/Blueprints/Game/BPRiotHUD.ClickedLocation` (`self.ClickedLocation`) _gamehudref)
          (set `self.SingleClick` false)
          (`KismetSystemLibrary.PrintString` (`KismetStringLibrary.Conv_IntToString` (`KismetArrayLibrary.Array_Length` (`self.PreselectedUnits`)))))))))

(event `PlaceSelectPressed`
  (bind (_locationx _locationy) (`self.GetMousePosition`))
  (set `self.SingleClick` true)
  (set `self.ClickedLocation` (`KismetMathLibrary.MakeVector2D` _locationx _locationy))
  (goto _label :!via `Open`))

(event `PlaceSelectReleased`
  (if (`self.SingleClick`)
    (`self.CheckForSelectedActor` false))
  (set `/Game/Blueprints/Game/BPRiotHUD.IsDrawing` false (`self.GameHUDRef`))
  (goto _label :!via `Close`))

(event `InputAction|Deselect`
  (params (Key :type "Key Structure" :default "AnyKey"))
  (:`Pressed`
    (`self.FinishRoad`)))

(fn `CheckForSelectedActor`
  (params (HitResult :type Boolean)))

(fn `MovementSpeedCalc`
  (returns (MouseSensitivity :type "Float (double-precision)"))
  (return (`KismetMathLibrary.FClamp` (/ (`SpringArmComponent.TargetArmLength` (`/Game/Blueprints/Player/BPRiotPawn.SpringArm` (`self.PlayerPawnRef`))) 100.0) 5.0 20.0)))

(fn `PlaceNewBuilding`
  (params (Locaction :type "Vector Structure"))
  (returns (Success :type Boolean))
  (bind _roads (`self.Roads`))
  (bind _asbproad_preview (cast `/Game/Blueprints/Preview/BPRoadPreview` (`self.Preview`) :!pure true))
  (bind _roadspline (`/Game/Blueprints/Preview/BPRoadPreview.RoadSpline` _asbproad_preview))
  (if (`self.BuildingEnabled`)
    ;[1 0.15 0.15] 2do HARDCODES need to fix
    (switch `/Game/ENums/Enum_GameMode` "NewEnumerator1"
      (:`NewEnumerator1`
        (switch `int` (`self.RoadMode`)
          (:`0`
            (`/Game/Blueprints/Preview/BPRoadPreview.SetStartPoint` _asbproad_preview Locaction)
            (set `self.RoadMode` 1)
            (`self.CreateRoad`))
          (:`1`
            (set `self.RoadMode` 2))
          (:`2`
            (set `self.RoadMode` 1)
            (`/Game/Blueprints/Preview/BPRoadPreview.SpawnRoad` _asbproad_preview (`|GetArrayItem` _roads (`KismetArrayLibrary.Array_LastIndex` _roads)))
            (`/Game/Blueprints/Preview/BPRoadPreview.SetStartPoint` _asbproad_preview (`SplineMeshComponent.GetEndPosition` _roadspline))
            (`/Game/Blueprints/Preview/BPRoadPreview.SetStartTangent` _asbproad_preview (* (`KismetMathLibrary.Normal` (`SplineMeshComponent.GetEndTangent` _roadspline)) 2000.0))))
        (return true))
      (:`NewEnumerator3`
        _)))
  (return false))

(fn `UserConstructionScript`)