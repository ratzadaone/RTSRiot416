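; Lumberjack industrial building that bids for a resource job and assigns employees to a work site.
; A second after BeginPlay it bids as Miner through the game state's BidManager, storing a won deposit as CurrentJobDeposit.
; AssignEmployeeJob instead reads CurrentJobSite, set by SetCurrentJob, and returns its entrance location to listed employees.
; Entering and exiting both resume stamina depletion, clear regeneration and call SwitchSleep on the NPC's controller.
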(event `self.ReceiveBeginPlay`
  (`parent.ReceiveBeginPlay`)
  ;[1 1 1] No delay will check before added to game
  (`KismetSystemLibrary.Delay` 1.0)
  (`self.BidForJob` "NewEnumerator2"))

(event `self.ReceiveTick`
  (params (DeltaSeconds :type "Float (single-precision)"))
  (`parent.ReceiveTick` DeltaSeconds))

(fn `AssignEmployeeJob`
  (params (Employee :type "/Game/Blueprints/Units/BPMasterHumanChar Object Reference"))
  (returns (JobAsigned :type Boolean) (JobInstance :type "Actor Object Reference") (JobLocation :type "Vector Structure"))
  (bind _currentjobsite (`self.CurrentJobSite`))
  ;[1 1 1] TO Check
  (if (and (!= (`KismetArrayLibrary.Array_Find` (`self.Employees`) Employee) -1) (`KismetSystemLibrary.IsValid` (`self.CurrentJobSite`)))
    (return true _currentjobsite (`SceneComponent.K2_GetComponentLocation` (`/Game/Blueprints/Buildings/BPBuildingMaster.Entrance` _currentjobsite)))
    (else
      (return false null (0.0 0.0 0.0)))))

(fn `BidForJob`
  (params (JobType :type "/Game/ENums/Enum_OcupationType Enum"))
  (returns (BidSuccess :type Boolean))
  (locals (JobDeposit_Loc :type "/Game/Blueprints/Resources/BPMasterDeposit Object Reference"))
  (if (`self.GetJobStatus` JobType)
    (return false)
    (else
      (switch `/Game/ENums/Enum_OcupationType` JobType
        (:`NewEnumerator2`
          (bind (_wonbid _jobsite) (`/Game/Blueprints/Game/BPRiotGameState.BidManager` (`self.GameStateRef`) self JobType "NewEnumerator1"))
          (if _wonbid
            (bind _output_get (set `self.CurrentJobDeposit` (cast `/Game/Blueprints/Resources/BPMasterDeposit` _jobsite :!pure true)))
            (`KismetSystemLibrary.PrintString` (`KismetStringLibrary.Concat_StrStr` "Mine set job deposit to  " (`KismetSystemLibrary.GetObjectName` _output_get)))
            (return true)
            (else
              (return false))))))))

(fn `EnterBuilding`
  (params (NPC :type "/Game/Blueprints/Units/BPMasterHumanChar Object Reference"))
  (returns (Success :type Boolean))
  (bind _aicontrollerref (`/Game/Blueprints/Units/BPMasterHumanChar.AIControllerRef` NPC))
  (`KismetSystemLibrary.K2_UnPauseTimerHandle` (`/Game/Blueprints/Units/BPAIControllerHumanChar.StaminaDepleteHandle` _aicontrollerref))
  (`KismetSystemLibrary.K2_ClearAndInvalidateTimerHandle` (`/Game/Blueprints/Units/BPAIControllerHumanChar.StaminaRegenHandle` _aicontrollerref))
  (`/Game/Blueprints/Units/BPAIControllerHumanChar.SwitchSleep` _aicontrollerref)
  (return true))

(fn `ExitBuilding`
  (params (NPC :type "/Game/Blueprints/Units/BPMasterHumanChar Object Reference"))
  (returns (Success :type Boolean))
  (bind _aicontrollerref (`/Game/Blueprints/Units/BPMasterHumanChar.AIControllerRef` NPC))
  (`KismetSystemLibrary.K2_UnPauseTimerHandle` (`/Game/Blueprints/Units/BPAIControllerHumanChar.StaminaDepleteHandle` _aicontrollerref))
  (`KismetSystemLibrary.K2_ClearAndInvalidateTimerHandle` (`/Game/Blueprints/Units/BPAIControllerHumanChar.StaminaRegenHandle` _aicontrollerref))
  (`/Game/Blueprints/Units/BPAIControllerHumanChar.SwitchSleep` _aicontrollerref)
  (return false))

(fn `SetCurrentJob`
  (params (JobSite :type "/Game/Blueprints/Buildings/BPBuildingMaster Object Reference"))
  (set `self.CurrentJobSite` JobSite)
  (return))

(fn `UserConstructionScript`
  (`parent.UserConstructionScript`))