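; Construction office building that bids for construction jobs and assigns its employees to the resulting job site.
; A looping timer triggers bidding while occupied, querying the GameState's BidManager unless job status blocks it, and pauses after a win.
; The won site becomes the current job, whose entrance location is handed to listed employees.
; Entering and exiting both resume NPC stamina depletion, clear regeneration and call SwitchSleep.
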(event `self.ReceiveBeginPlay`
  (`parent.ReceiveBeginPlay`)
  (bind _returnvalue (`KismetSystemLibrary.K2_SetTimerDelegate` (`|CreateDelegate` :!event `BidTimerEventOffice`) 1.0 true))
  (set `self.BidTimerHandleOffice` _returnvalue))

(event `BidTimerEventOffice`
  (`KismetSystemLibrary.PrintString` "OfficeBidding")
  (if (`self.GetOccupants`)
    (bind _bidsuccess (`self.BidForJob` "NewEnumerator1"))
    (if _bidsuccess
      (`KismetSystemLibrary.K2_PauseTimerHandle` (`self.BidTimerHandleOffice`)))))

(fn `AssignEmployeeJob`
  (params (Employee :type "/Game/Blueprints/Units/BPMasterHumanChar Object Reference"))
  (returns (JobAsigned :type Boolean) (JobInstance :type "Actor Object Reference") (JobLocation :type "Vector Structure"))
  (bind _currentjobsite (`self.CurrentJobSite`))
  (if (and (!= (`KismetArrayLibrary.Array_Find` (`self.Employees`) Employee) -1) (`KismetSystemLibrary.IsValid` (`self.CurrentJobSite`)))
    (return true _currentjobsite (`SceneComponent.K2_GetComponentLocation` (`/Game/Blueprints/Buildings/BPBuildingMaster.Entrance` _currentjobsite)))
    (else
      (return false null (0.0 0.0 0.0)))))

(fn `BidForJob`
  (params (JobType :type "/Game/ENums/Enum_OcupationType Enum"))
  (returns (BidSuccess :type Boolean))
  (locals (JobSite_Loc :type "/Game/Blueprints/Buildings/BPBuildingMaster Object Reference"))
  (`KismetSystemLibrary.PrintString` "ConstructionOfficeBidding")
  (if (`self.GetJobStatus` JobType)
    (return false)
    (else
      (switch `/Game/ENums/Enum_OcupationType` JobType
        (:`NewEnumerator1`
          (bind (_wonbid _jobsite) (`/Game/Blueprints/Game/BPRiotGameState.BidManager` (`self.GameStateRef`) self))
          (set `local.JobSite_Loc` _jobsite)
          (if _wonbid
            (set `self.CurrentJobSite` (`local.JobSite_Loc`))
            (return true)
            (else
              (return false))))))))

(fn `EnterBuilding`
  (params (NPC :type "/Game/Blueprints/Units/BPMasterHumanChar Object Reference"))
  (returns (Success :type Boolean))
  (bind _aicontrollerref (`/Game/Blueprints/Units/BPMasterHumanChar.AIControllerRef` NPC))
  (`KismetSystemLibrary.K2_UnPauseTimerHandle` (`/Game/Blueprints/Units/BPAIControllerHumanChar.StaminaDepleteHandle` _aicontrollerref))
  (`KismetSystemLibrary.K2_ClearAndInvalidateTimerHandle` (`/Game/Blueprints/Units/BPAIControllerHumanChar.StaminaRegenHandle` _aicontrollerref))
  (`/Game/Blueprints/Units/BPAIControllerHumanChar.SwitchSleep` _aicontrollerref)
  (return true))

(fn `ExitBuilding`
  (params (NPC :type "/Game/Blueprints/Units/BPMasterHumanChar Object Reference"))
  (returns (Success :type Boolean))
  (bind _aicontrollerref (`/Game/Blueprints/Units/BPMasterHumanChar.AIControllerRef` NPC))
  (`KismetSystemLibrary.K2_UnPauseTimerHandle` (`/Game/Blueprints/Units/BPAIControllerHumanChar.StaminaDepleteHandle` _aicontrollerref))
  (`KismetSystemLibrary.K2_ClearAndInvalidateTimerHandle` (`/Game/Blueprints/Units/BPAIControllerHumanChar.StaminaRegenHandle` _aicontrollerref))
  (`/Game/Blueprints/Units/BPAIControllerHumanChar.SwitchSleep` _aicontrollerref)
  (return false))

(fn `SetCurrentJob`
  (params (JobSite :type "/Game/Blueprints/Buildings/BPBuildingMaster Object Reference"))
  (set `self.CurrentJobSite` JobSite)
  (return))

(fn `UserConstructionScript`
  (`parent.UserConstructionScript`))