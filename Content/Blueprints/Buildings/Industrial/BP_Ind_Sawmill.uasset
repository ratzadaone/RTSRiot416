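; BP_Ind_Sawmill is an industrial sawmill building that adjusts an NPC's stamina state when it enters or exits.
; EnterBuilding and ExitBuilding both unpause the AI controller's stamina depletion timer, clear its regeneration timer and call SwitchSleep.
; The two functions differ only in their return value: true on enter, false on exit.
; The event graph holds only disabled stubs and the construction script only calls its parent.
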(fn `EnterBuilding`
  (params (NPC :type "/Game/Blueprints/Units/BPMasterHumanChar Object Reference"))
  (returns (Success :type Boolean))
  (bind _aicontrollerref (`/Game/Blueprints/Units/BPMasterHumanChar.AIControllerRef` NPC))
  (`KismetSystemLibrary.K2_UnPauseTimerHandle` (`/Game/Blueprints/Units/BPAIControllerHumanChar.StaminaDepleteHandle` _aicontrollerref))
  (`KismetSystemLibrary.K2_ClearAndInvalidateTimerHandle` (`/Game/Blueprints/Units/BPAIControllerHumanChar.StaminaRegenHandle` _aicontrollerref))
  (`/Game/Blueprints/Units/BPAIControllerHumanChar.SwitchSleep` _aicontrollerref)
  (return true))

(fn `ExitBuilding`
  (params (NPC :type "/Game/Blueprints/Units/BPMasterHumanChar Object Reference"))
  (returns (Success :type Boolean))
  (bind _aicontrollerref (`/Game/Blueprints/Units/BPMasterHumanChar.AIControllerRef` NPC))
  (`KismetSystemLibrary.K2_UnPauseTimerHandle` (`/Game/Blueprints/Units/BPAIControllerHumanChar.StaminaDepleteHandle` _aicontrollerref))
  (`KismetSystemLibrary.K2_ClearAndInvalidateTimerHandle` (`/Game/Blueprints/Units/BPAIControllerHumanChar.StaminaRegenHandle` _aicontrollerref))
  (`/Game/Blueprints/Units/BPAIControllerHumanChar.SwitchSleep` _aicontrollerref)
  (return false))

(fn `UserConstructionScript`
  (`parent.UserConstructionScript`))