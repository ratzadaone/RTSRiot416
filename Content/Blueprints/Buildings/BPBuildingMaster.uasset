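; Base Blueprint for game buildings, configured from a data table row, with hiring, shifts, night lights, hover highlighting, unit spawning and stub occupancy functions for children.
; On spawn it deducts resources and joins the build queue.
; Tick scales a timeline by active workers while materials remain, driving a height-based swipe material and consuming materials.
; Completion swaps material and gameplay tags, frees workers and contractor, and updates the selected building's HUD.
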(event `self.ReceiveActorBeginOverlap`
  (params (OtherActor :type "Actor Object Reference")))

(event `self.ReceiveTick`
  (params (DeltaSeconds :type "Float (single-precision)"))
  (bind _activeworkers (`self.GetWorkForceNr`))
  ;[0.984 1 1] Construction Tick
  (if (> _activeworkers 0.0)
    (`TimelineComponent.SetPlayRate` (`self.FadeMaterial`) (* (/ 1.0 (* (`.BuildingRequiredHours_42_848ADDA2447040C752E97386F2554355` (break `/Game/Structs/Building_Properties_Struct` (`self.BuildingStructFromTable`))) 60.0)) _activeworkers))
    (if (> (`BlueprintMapLibrary.Map_Length` (`self.MaterialsForConstruction`)) 0)
      (`TimelineComponent.Play` (`self.FadeMaterial`))
      (else
        (`TimelineComponent.Stop` (`self.FadeMaterial`))))
    (else
      (`TimelineComponent.Stop` (`self.FadeMaterial`)))))

(event `OnSpawned`
  (bind (_returnvalue_x _returnvalue_y _returnvalue_z) (`KismetMathLibrary.BreakVector` (`self.K2_GetActorLocation`)))
  (bind _returnvalue (`StaticMesh.GetBounds` (`StaticMeshComponent.StaticMesh` (`self.StaticMesh`))))
  ;[1 1 1] OnSpawned
  (bind _success (`self.fnDeductResources` false))
  (if _success
    (`self.fnCalculatePercentMaterialUnit`)
    (`KismetArrayLibrary.Array_Add` (`/Game/Blueprints/Game/BPRiotGameState.BuildingQueue` (`self.GameStateRef`)) self)
    (bind _returnvalue_2 (`PrimitiveComponent.CreateDynamicMaterialInstance` (`self.StaticMesh`) 0 "/Game/Materials/Swipe.Swipe"))
    (`MaterialInstanceDynamic.SetScalarParameterValue` _returnvalue_2 "Height" (- (+ (.z (`KismetMathLibrary.BreakBoxSphereBounds` _returnvalue)) (.z (`.BoxExtent` (`KismetMathLibrary.BreakBoxSphereBounds` _returnvalue)))) _returnvalue_z))
    (`MaterialInstanceDynamic.SetScalarParameterValue` _returnvalue_2 "Height" (- (+ (.z (`KismetMathLibrary.BreakBoxSphereBounds` _returnvalue)) (.z (`.BoxExtent` (`KismetMathLibrary.BreakBoxSphereBounds` _returnvalue)))) _returnvalue_z))
    (`MaterialInstanceDynamic.SetScalarParameterValue` _returnvalue_2 "StartingOffset" (- (- (.z (`KismetMathLibrary.BreakBoxSphereBounds` _returnvalue)) (.z (`.BoxExtent` (`KismetMathLibrary.BreakBoxSphereBounds` _returnvalue)))) _returnvalue_z))
    (bind _output_get (set `self.GameplayTagContainer` (`BlueprintGameplayTagLibrary.MakeLiteralGameplayTagContainer` (struct :`GameplayTags` (struct :`(TagName` "building"))))))
    (`BlueprintGameplayTagLibrary.AddGameplayTag` _output_get (struct :`TagName` "building.in_construction"))
    (else
      (`self.K2_DestroyActor`)
      (set `/Game/Blueprints/Player/BPRiotController.GameMode` "NewEnumerator3" (`self.ControllerRef`))
      (`KismetSystemLibrary.PrintString` "Fix Here Readd Preview" true true (struct :`R` 1.0 :`G` 0.249349 :`B` 0.279199 :`A` 1.0) 20.0))))

(event `self.ReceiveBeginPlay`
  ;[1 1 1] BeginPlay
  (`/Engine/EditorBlueprintResources/StandardMacros.IsValid` (`self.ControllerRef`)
    (:`Is Valid`
      _)
    (:`Is Not Valid`
      (bind _asbpriot_controller (cast `/Game/Blueprints/Player/BPRiotController` (`GameplayStatics.GetPlayerController` 0)))
      (set `self.ControllerRef` _asbpriot_controller)))
  (`/Engine/EditorBlueprintResources/StandardMacros.IsValid` (`self.GameStateRef`)
    (:`Is Valid`
      _)
    (:`Is Not Valid`
      (set `self.GameStateRef` (cast `/Game/Blueprints/Game/BPRiotGameState` (`GameplayStatics.GetGameState`) :!pure true))))
  (`/Game/Blueprints/Game/BPRiotGameState.AddBuildingsToGame` (`self.GameStateRef`) self)
  (`KismetSystemLibrary.Delay` 1.0)
  (add `/Game/Blueprints/Game/BPRiotGameState.LightsOn` (`self.GameStateRef`) (delegate `LightsOn`)))

(event `LightsOn`
  (params (TurnOn :type Boolean))
  (bind _buildinglight (`self.BuildingLight`))
  ;[1 1 1] BeginPlay
  (if TurnOn
    (`KismetSystemLibrary.Delay` (`KismetMathLibrary.RandomFloatInRange` 0.0 2.0))
    (`LightComponent.SetIntensity` _buildinglight 20000.0)
    (else
      (`KismetSystemLibrary.Delay` (`KismetMathLibrary.RandomFloatInRange` 0.0 2.0))
      (`LightComponent.SetIntensity` _buildinglight 0.0))))

(event `SpawnHumanUnit`
  (bind _staticmesh (`self.StaticMesh`))
  (bind (_returnvalue_location _returnvalue_rotation) (`KismetMathLibrary.BreakTransform` (`SceneComponent.K2_GetComponentToWorld` _staticmesh)))
  (bind (_returnvalue_x _returnvalue_y _returnvalue_z) (`KismetMathLibrary.BreakVector` (`SceneComponent.GetRightVector` _staticmesh)))
  ;[1 1 1] SpawnHuman
  (bind _returnvalue (`|SpawnActorFromClass` "/Game/Blueprints/Units/BPMasterHumanChar.BPMasterHumanChar_C" (`KismetMathLibrary.MakeTransform` (+ _returnvalue_location (`KismetMathLibrary.MakeVector` _returnvalue_x (* _returnvalue_y 1200.0) (+ _returnvalue_z 250.0))) _returnvalue_rotation) "AlwaysSpawn" "OverrideRootScale"))
  (`NavigationSystem.SimpleMoveToLocation` (`Pawn.GetController` _returnvalue) (`SceneComponent.K2_GetComponentLocation` (`self.RallyPointDecal`))))

(event `self.StaticMesh.OnBeginCursorOver`
  (params (TouchedComponent :type "PrimitiveComponent Object Reference"))
  ;[1 1 1] MouseOver
  (`PrimitiveComponent.SetRenderCustomDepth` (`self.StaticMesh`) true))

(event `self.StaticMesh.OnEndCursorOver`
  (params (TouchedComponent :type "PrimitiveComponent Object Reference"))
  ;[1 1 1] MouseOver
  (`PrimitiveComponent.SetRenderCustomDepth` (`self.StaticMesh`) false))

(fn `AssignEmployeeJob`
  (params (Employee :type "/Game/Blueprints/Units/BPMasterHumanChar Object Reference"))
  (returns (JobAsigned :type Boolean) (JobInstance :type "Actor Object Reference") (JobLocation :type "Vector Structure"))
  ;[1 1 1] Function to be overriden by children blueprints
  (return false null (0.0 0.0 0.0)))

(fn `DestroySelf`
  (switch `/Game/ENums/Enum_BuildingCategory` (`.BuildingCategory_17_565F2E76468F1F6C36BD80A8E9D51E51` (break `/Game/Structs/Building_Properties_Struct` (`self.BuildingStructFromTable`)))
    (:`NewEnumerator0`
      (for _array_element (`self.Residents`)
        (bind _aicontrollerref (`/Game/Blueprints/Units/BPMasterHumanChar.AIControllerRef` _array_element))
        (bind _payed (`/Game/Blueprints/Units/BPAIControllerHumanChar.PayRent` _aicontrollerref true))
        (if _payed
          (bind _returnvalue (`AIBlueprintHelperLibrary.GetBlackboard` _aicontrollerref))
          (`BlackboardComponent.SetValueAsEnum` _returnvalue "AI_State" (enumliteral `/Game/ENums/Enum_AI_State` "NewEnumerator0"))
          (`BlackboardComponent.SetValueAsObject` _returnvalue "HouseReference" null)
          (`BlackboardComponent.ClearValue` _returnvalue "CurrentLocation")
          (`BlueprintMapLibrary.Map_Remove` (`/Game/Blueprints/Game/BPRiotGameState.BuildingsInGame` (`self.GameStateRef`)) self)
          (`self.K2_DestroyActor`))))))

(fn `EnterBuilding`
  (params (NPC :type "/Game/Blueprints/Units/BPMasterHumanChar Object Reference"))
  (returns (Success :type Boolean))
  (return false))

(fn `ExitBuilding`
  (params (NPC :type "/Game/Blueprints/Units/BPMasterHumanChar Object Reference"))
  (returns (Success :type Boolean))
  (return false))

(fn `fnCalculatePercentMaterialUnit`
  (locals (TempToAdd_Loc :type Integer :default 0))
  (for _array_element (`.BuildingRequiredResources_43_16ECF3C946C5ABD7F8FEC59BAF30D635` (break `/Game/Structs/Building_Properties_Struct` (`self.BuildingStructFromTable`)))
    (set `local.TempToAdd_Loc` (+ (`.ResIndexAmount_5_7059E5C3465FB29D23AFC48B9314045B` (break `/Game/Structs/STRUCT_ResourcesIndexes` _array_element)) (`local.TempToAdd_Loc`))))
  (bind _output_get (set `self.ConsumeUnitPercent` (/ 1.0 (`KismetMathLibrary.Conv_IntToDouble` (`local.TempToAdd_Loc`)))))
  (`KismetSystemLibrary.PrintString` (`KismetStringLibrary.Concat_StrStr` "Consume Percent" " " (`KismetStringLibrary.Conv_IntToString` (`local.TempToAdd_Loc`)) " " (`KismetStringLibrary.Conv_DoubleToString` _output_get))))

(fn `fnConsumeMaterials`
  (locals (AmountToAdd_Loc :type Integer :default 0) (PercentPerUnit :type "Float (double-precision)" :default 0.0) (OrigAmount :type "Float (double-precision)" :default 0.0) (NewLocalVar_0 :type "Map of /Game/ENums/Enum_ResourcesROwNames Enum to Float (double-precision)"))
  (bind _materialsforconstruction (`self.MaterialsForConstruction`))
  (bind _materialsforconstruction_2 (`self.MaterialsForConstruction`))
  (bind _materialsforconstruction_3 (`self.MaterialsForConstruction`))
  (bind _returnvalue (`BlueprintMapLibrary.Map_Length` _materialsforconstruction_3))
  (bind _returnvalue_2 (- (`self.TempAmountToConsume`) (* (- 1.0 (`self.ConsumeUnitPercent`)) (* (`self.TimelinePos`) 100.0))))
  (bind _keys (`BlueprintMapLibrary.Map_Keys` _materialsforconstruction))
  (if (== (`self.TempAmountToConsume`) 0.0)
    (bind _output (`|GetArrayItem` _keys))
    (bind _output_get (set `self.TempAmountToConsume` (+ (`BlueprintMapLibrary.Map_Find` _materialsforconstruction _output) (`self.TempToAdd`))))
    (`KismetSystemLibrary.PrintString` (`KismetStringLibrary.Concat_StrStr` "To consume IS " (`KismetStringLibrary.Conv_DoubleToString` _output_get)) true true (struct :`G` 0.66 :`B` 1.0 :`A` 1.0) 50.0))
  (`BlueprintMapLibrary.Map_Add` _materialsforconstruction _output _returnvalue_2)
  (`KismetSystemLibrary.PrintString` (`KismetStringLibrary.Concat_StrStr` (`KismetStringLibrary.Conv_DoubleToString` _returnvalue_2) " " (`KismetStringLibrary.Conv_DoubleToString` (* (- 1.0 (`self.TimelinePos`)) 100.0))) true true (struct :`G` 0.66 :`B` 1.0 :`A` 1.0) 50.0)
  (if (<= _returnvalue_2 0.0)
    (bind _returnvalue_3 (`BlueprintMapLibrary.Map_Remove` _materialsforconstruction_3 (cast `/Game/ENums/Enum_ResourcesROwNames` _output)))
    (set `self.TempToAdd` (+ (`self.TempToAdd`) (`self.TempAmountToConsume`)))
    (set `self.TempAmountToConsume` 0.0)
    (`KismetSystemLibrary.PrintString` (`KismetStringLibrary.Concat_StrStr` "Length left " (`KismetStringLibrary.Conv_IntToString` _returnvalue) " " (`KismetStringLibrary.Conv_BoolToString` _returnvalue_3)) true true (struct :`G` 0.66 :`B` 1.0 :`A` 1.0) 20.0)
    (bind _keys_2 (`BlueprintMapLibrary.Map_Keys` _materialsforconstruction_2))
    (for (_array_element _array_index) _keys_2
      (`KismetSystemLibrary.PrintString` (`KismetStringLibrary.Concat_StrStr` "Keys left: " (`|GetEnumeratorNameAsString` _array_element) "Index " (`KismetStringLibrary.Conv_IntToString` _array_index) "Value: " (`KismetStringLibrary.Conv_DoubleToString` (`BlueprintMapLibrary.Map_Find` _materialsforconstruction_2 _array_element))) true true (struct :`G` 0.66 :`B` 1.0 :`A` 1.0) 50.0))
    (if (> _returnvalue 0)
      (`self.fnConsumeMaterials`)
      (return)
      (else
        (`KismetSystemLibrary.PrintString` "LENGTH IS 0" true true (struct :`R` 1.0 :`G` 0.464275 :`B` 0.701468 :`A` 1.0) 50.0)
        (return)))
    (else
      (return))))

(fn `fnDeductResources`
  (params (Refund :type Boolean))
  (returns (Success :type Boolean))
  (locals (Success_Loc :type Boolean :default true))
  (bind _resourcelist (`/Game/Blueprints/Player/BPRiotController.ResourceList` (`self.ControllerRef`)))
  (for _array_element (`.BuildingRequiredResources_43_16ECF3C946C5ABD7F8FEC59BAF30D635` (break `/Game/Structs/Building_Properties_Struct` (`self.BuildingStructFromTable`)))
    (if Refund
      (bind (_resindex _resindexamount) (break `/Game/Structs/STRUCT_ResourcesIndexes` _array_element))
      (bind _value (`BlueprintMapLibrary.Map_Find` _resourcelist _resindex))
      (`BlueprintMapLibrary.Map_Add` _resourcelist _resindex (+ _value _resindexamount))
      (else
        (`BlueprintMapLibrary.Map_Add` _resourcelist _resindex (- _value _resindexamount))))
    (`TextBlock.SetText` (`/Game/Blueprints/Widgets/WidgetElements/ResourceInfo.ResourceText` (`BlueprintMapLibrary.Map_Find` (`/Game/Blueprints/Widgets/WMainUI.ResWidgetsMap` (`/Game/Blueprints/Player/BPRiotController.WidgetHUDRef` (`self.ControllerRef`))) _resindex)) (`KismetTextLibrary.Conv_IntToText` _value)))
  (return (`local.Success_Loc`)))

(fn `GetOccupants`
  (returns (HasOccupants :type Boolean) (NrOfOccupants :type Integer) (ListOfOccupants :type "Array of /Game/Blueprints/Units/BPMasterHumanChar Object Reference"))
  (return false 0))

(fn `GetWorkForceNr`
  (returns (ActiveWorkers :type "Float (double-precision)"))
  (return (`KismetMathLibrary.Conv_IntToDouble` (`KismetArrayLibrary.Array_Length` (`self.ActiveWorkers`)))))

(fn `HireEmployee`
  (params (NPC :type "/Game/Blueprints/Units/BPMasterHumanChar Object Reference"))
  (returns (WasHired :type Boolean) (HiringBuilding :type "/Game/Blueprints/Buildings/BPBuildingMaster Object Reference"))
  (locals (Applicant_Loc :type "/Game/Blueprints/Units/BPMasterHumanChar Object Reference"))
  (set `local.Applicant_Loc` NPC)
  (if (< (`.NrOfOccupants` (`self.GetOccupants`)) (`.BuildingMaxEmployees_26_52DD647444C16E30BA0F78B0E3BFA0F2` (break `/Game/Structs/Building_Properties_Struct` (`self.BuildingStructFromTable`))))
    (`KismetArrayLibrary.Array_AddUnique` (`self.Employees`) (`local.Applicant_Loc`))
    (return true self)
    (else
      (return false null))))

(fn `LeaveShift`
  (params (Employee :type "/Game/Blueprints/Units/BPMasterHumanChar Object Reference"))
  (returns (HasToExit :type Boolean))
  (if (> (`KismetArrayLibrary.Array_Find` (`self.ActiveWorkers`) Employee) -1)
    (bind _returnvalue (`KismetArrayLibrary.Array_RemoveItem` (`self.ActiveWorkers`) Employee))
    (return _returnvalue)
    (else
      (return false))))

(fn `ReportToShift`
  (params (Worker :type "/Game/Blueprints/Units/BPMasterHumanChar Object Reference"))
  (`KismetArrayLibrary.Array_Add` (`self.ActiveWorkers`) Worker)
  (set `/Game/Blueprints/Units/BPMasterHumanChar.LastWorkingLocation` (`SceneComponent.K2_GetComponentLocation` (`self.Entrance`)) Worker)
  (return))

(fn `UserConstructionScript`
  (locals (EntranceDistance :type "Float (double-precision)" :default 150.0))
  (bind _collision (`self.Collision`))
  (bind _min (`StaticMeshComponent.GetLocalBounds` (`self.StaticMesh`)))
  (bind _returnvalue (`|GetDataTableRow` "/Game/DataTables/DT_Buildings.DT_Buildings" (`KismetStringLibrary.Conv_StringToName` (`|GetEnumeratorNameAsString` (`self.BuildingIndex`))))
    (:`then`
      (set `self.BuildingStructFromTable` _returnvalue)
      (`SceneComponent.K2_SetRelativeLocation` (`self.Entrance`) (`KismetMathLibrary.MakeVector` 0.0 (+ (`KismetMathLibrary.Abs` (.y (`StaticMeshComponent.GetLocalBounds` (`self.StaticMesh`)))) (`local.EntranceDistance`)) 50.0) false false)
      (`BoxComponent.SetBoxExtent` _collision (`KismetMathLibrary.MakeVector` (- (`KismetMathLibrary.Abs` (.x _min)) 20.0) 98.0 10.0) true)
      (`SceneComponent.K2_SetRelativeLocation` _collision (`KismetMathLibrary.MakeVector` 0.0 (+ (`KismetMathLibrary.Abs` (.y _min)) 98.0) 10.0) false false))))