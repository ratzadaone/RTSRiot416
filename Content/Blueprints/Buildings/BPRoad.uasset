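; BPRoad is a road building actor that grows a spline one section at a time and covers it with textured road meshes.
; AddSpline sets the last point's location and leave tangent, then appends the new end point.
; CreateMeshBetweenPoints lays fixed-length spline mesh segments with dynamic materials.
; Only the newest section's meshes are cached, so each addition destroys and rebuilds the previous section before meshing the new one.
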(event `Create`
  (params (`Object ID` :type String))
  (set `self.ID` `Object ID`))

(event `AddSpline`
  (params (StartPosition :type "Vector Structure") (StartTangent :type "Vector Structure") (EndPosition :type "Vector Structure") (EndTangent :type "Vector Structure"))
  (bind _roadspline (`self.RoadSpline`))
  (bind _returnvalue (- (`SplineComponent.GetNumberOfSplinePoints` (`self.RoadSpline`)) 1))
  (bind _returnvalue_2 (- _returnvalue 2))
  (bind _returnvalue_3 (- _returnvalue 1))
  (`SplineComponent.SetLocationAtSplinePoint` _roadspline _returnvalue StartPosition "World" false)
  (`SplineComponent.SetTangentsAtSplinePoint` _roadspline _returnvalue (`SplineComponent.GetArriveTangentAtSplinePoint` (`self.RoadSpline`) _returnvalue "Local") StartTangent "World" false)
  (`SplineComponent.AddSplinePoint` _roadspline EndPosition "World" false)
  (`SplineComponent.SetTangentAtSplinePoint` _roadspline _returnvalue EndTangent "World" true)
  (`self.DestroyCachedRoad`)
  (if (> _returnvalue_2 -1)
    (`self.CreateMeshBetweenPoints` _returnvalue_2 _returnvalue_3 150.0))
  (`self.CreateMeshBetweenPoints` _returnvalue_3 _returnvalue 150.0 true))

(fn `CreateMeshBetweenPoints`
  (params (Start :type Integer) (End :type Integer) (`Segment Length` :type "Float (double-precision)") (AddToCachedRoad :type Boolean))
  (bind _roadspline (`self.RoadSpline`))
  (bind _roadspline_2 (`self.RoadSpline`))
  (bind _returnvalue (`SplineComponent.GetDistanceAlongSplineAtSplinePoint` _roadspline Start))
  (for _index (range (+ (`.ReturnValue` (`KismetMathLibrary.FMod` (- (`SplineComponent.GetDistanceAlongSplineAtSplinePoint` _roadspline End) _returnvalue) `Segment Length`)) 1))
    (bind _returnvalue_2 (`AddComponent|NODE_AddSplineMeshComponent-2`))
    (bind _returnvalue_3 (+ _returnvalue (* _index `Segment Length`)))
    (bind _returnvalue_4 (+ _returnvalue_3 `Segment Length`))
    (`SplineMeshComponent.SetStartAndEnd` _returnvalue_2 (`SplineComponent.GetLocationAtDistanceAlongSpline` _roadspline_2 _returnvalue_3 "World") (* (`SplineComponent.GetDirectionAtDistanceAlongSpline` _roadspline_2 _returnvalue_3 "World") `Segment Length`) (`SplineComponent.GetLocationAtDistanceAlongSpline` _roadspline_2 _returnvalue_4 "World") (* (`SplineComponent.GetDirectionAtDistanceAlongSpline` _roadspline_2 _returnvalue_4 "World") `Segment Length`) true)
    (`StaticMeshComponent.SetStaticMesh` _returnvalue_2 "/Game/Mesh/m_road.m_road")
    (bind _returnvalue_5 (`PrimitiveComponent.CreateDynamicMaterialInstance` _returnvalue_2 0 "/Game/Materials/s_custom.s_custom"))
    (`MaterialInstanceDynamic.SetTextureParameterValue` _returnvalue_5 "Texture" "/Game/Textures/T_road.T_road")
    (if AddToCachedRoad
      (`KismetArrayLibrary.Array_Add` (`self.CachedRoad`) _returnvalue_2))))

(fn `DestroyCachedRoad`
  (bind _cachedroad (`self.CachedRoad`))
  (for _array_element _cachedroad
    (`/Engine/EditorBlueprintResources/StandardMacros.IsValid` _array_element
      (:`Is Valid`
        (`ActorComponent.K2_DestroyComponent` _array_element))))
  (`KismetArrayLibrary.Array_Clear` _cachedroad))

(fn `UserConstructionScript`)