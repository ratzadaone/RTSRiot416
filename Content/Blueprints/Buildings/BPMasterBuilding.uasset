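; Master building Blueprint for an RTS-style game, covering timed construction, unit spawning and cursor hover highlighting.
; OnSpawned drives a bounds-fitted Swipe material with a timeline scaled to BuildTime.
; On completion it swaps to a wall material, leaves the controller's in-progress list and, if selected, switches from construction to finished HUD.
; SpawnHumanUnit sends new units to the rally point decal, while hovering toggles custom depth rendering.
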(event `OnSpawned`
  (bind (_returnvalue_x _returnvalue_y _returnvalue_z) (`KismetMathLibrary.BreakVector` (`self.K2_GetActorLocation`)))
  (bind _controllerref (`self.ControllerRef`))
  (bind _staticmesh (`self.StaticMesh`))
  (bind _userwidgets (`/Game/Blueprints/Player/BPRiotController.UserWidgets` (`self.ControllerRef`)))
  (bind _returnvalue (`StaticMesh.GetBounds` (`StaticMeshComponent.StaticMesh` (`self.StaticMesh`))))
  (bind _returnvalue_2 (`PrimitiveComponent.CreateDynamicMaterialInstance` _staticmesh 0 "/Game/Materials/Swipe.Swipe"))
  (`MaterialInstanceDynamic.SetScalarParameterValue` _returnvalue_2 "Height" (- (+ (.z (`KismetMathLibrary.BreakBoxSphereBounds` _returnvalue)) (.z (`.BoxExtent` (`KismetMathLibrary.BreakBoxSphereBounds` _returnvalue)))) _returnvalue_z))
  (`MaterialInstanceDynamic.SetScalarParameterValue` _returnvalue_2 "StartingOffset" (- (- (.z (`KismetMathLibrary.BreakBoxSphereBounds` _returnvalue)) (.z (`.BoxExtent` (`KismetMathLibrary.BreakBoxSphereBounds` _returnvalue)))) _returnvalue_z))
  (`TimelineComponent.SetPlayRate` (`self.FadeMaterial`) (/ 1.0 (`self.BuildTime`)))
  (bind (_direction _amount) (`Timeline|FadeMaterial` :!via `PlayFromStart`)
    (:`Update`
      (`MaterialInstanceDynamic.SetScalarParameterValue` _returnvalue_2 "Amount" _amount))
    (:`Finished`
      (bind _returnvalue_3 (`PrimitiveComponent.CreateDynamicMaterialInstance` _staticmesh 0 "/Game/Materials/M_Basic_Wall.M_Basic_Wall"))
      (`MaterialInstanceDynamic.SetVectorParameterValue` _returnvalue_3 "Color" (struct :`R` 0.198866 :`G` 0.223303 :`B` 0.93 :`A` 1.0))
      (`KismetArrayLibrary.Array_RemoveItem` (`/Game/Blueprints/Player/BPRiotController.BuildingsInProgress` _controllerref) self)
      ;[1 1 1] MaybeRemove ?
      (set `self.IsFinished` true)
      (if (== self (`/Game/Blueprints/Player/BPRiotController.SelectedBuilding` _controllerref))
        (`Widget.SetVisibility` (`BlueprintMapLibrary.Map_Find` _userwidgets (`self.ConstructionHUD`)) "Hidden")
        (`Widget.SetVisibility` (`BlueprintMapLibrary.Map_Find` _userwidgets (`self.FinishedHUD`)) "SelfHitTestInvisible"))
      (`KismetSystemLibrary.PrintString` "Building Finished - HAVE TO FIX HUD" true true (struct :`R` 1.0 :`A` 1.0) 10.0))))

(event `self.ReceiveBeginPlay`
  (`/Engine/EditorBlueprintResources/StandardMacros.IsValid` (`self.ControllerRef`)
    (:`Is Not Valid`
      (bind _asbpriot_controller (cast `/Game/Blueprints/Player/BPRiotController` (`GameplayStatics.GetPlayerController` 0)))
      (set `self.ControllerRef` _asbpriot_controller))))

(event `SpawnHumanUnit`
  (bind _staticmesh (`self.StaticMesh`))
  (bind (_returnvalue_location _returnvalue_rotation) (`KismetMathLibrary.BreakTransform` (`SceneComponent.K2_GetComponentToWorld` _staticmesh)))
  (bind (_returnvalue_x _returnvalue_y _returnvalue_z) (`KismetMathLibrary.BreakVector` (`SceneComponent.GetRightVector` _staticmesh)))
  (bind _returnvalue (`|SpawnActorFromClass` "/Game/Blueprints/Units/BPMasterHumanChar.BPMasterHumanChar_C" (`KismetMathLibrary.MakeTransform` (+ _returnvalue_location (`KismetMathLibrary.MakeVector` _returnvalue_x (* _returnvalue_y 1200.0) (+ _returnvalue_z 250.0))) _returnvalue_rotation) "AlwaysSpawn" "OverrideRootScale"))
  (`NavigationSystem.SimpleMoveToLocation` (`Pawn.GetController` _returnvalue) (`SceneComponent.K2_GetComponentLocation` (`self.RallyPointDecal`))))

(event `self.StaticMesh.OnBeginCursorOver`
  (params (TouchedComponent :type "PrimitiveComponent Object Reference"))
  (`PrimitiveComponent.SetRenderCustomDepth` (`self.StaticMesh`) true))

(event `self.StaticMesh.OnEndCursorOver`
  (params (TouchedComponent :type "PrimitiveComponent Object Reference"))
  (`PrimitiveComponent.SetRenderCustomDepth` (`self.StaticMesh`) false))

(fn `UserConstructionScript`)